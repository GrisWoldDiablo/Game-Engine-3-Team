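; BP_CubeEnemyTest is a test cube enemy that loses a fixed bit of HP on any damage and destroys itself at zero.
; Tick feeds HP to its child-actor BP_Target_System and toggles the target arrow through a check against itself.
; FInisherCam uses a timeline to move CC0 along a spline, keeping it aimed at the enemy's root.
; The construction script places CC0 at the spline's first point, facing the root.
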(event Custom|FInisherCam
  (bind _cc_0 (Variables|Default|GetCC_0))
  (bind _spline_0 (Variables|Default|GetSpline_0))
  (bind _track_percentage (Timeline|Timeline_0_0 PlayFromStart)
    (:Update
      (Transformation|SetWorldTransform _cc_0 (Spline|GetTransformatDistanceAlongSpline _spline_0 (* _track_percentage (Spline|GetSplineLength _spline_0)) "World" false) false false)
      (Transformation|SetWorldRotation _cc_0 (Math|Rotator|FindLookatRotation (Transformation|GetWorldLocation _cc_0) (Transformation|GetWorldLocation (Variables|Transformation|GetRootComponent))) false false))))

(event EventTick
  (params (DeltaSeconds :type Float%20%28single-precision%29))
  (bind _targetarrow (Variables|Default|GetTargetArrow))
  (Variables|/Game/_Sarkis/Blueprint/BP_Target_System.BP_Target_System_C|Settest (Variables|Default|GetTargetSystem) (Variables|Default|GetHP))
  (if (== 0 self)
    (Rendering|SetVisibility _targetarrow true false)
    (else
      (Rendering|SetVisibility _targetarrow false false))))

(event Game|Damage|EventAnyDamage
  (params (Damage :type Float%20%28single-precision%29) (DamageType :type Damage%20Type%20Object%20Reference) (InstigatedBy :type Controller%20Object%20Reference) (DamageCauser :type Actor%20Object%20Reference))
  (Development|PrintString "Ouch!")
  (Variables|Default|SetHP (- (Variables|Default|GetHP) 0.1))
  (if (<= (Variables|Default|GetHP) 0.0)
    (Actor|DestroyActor)))

(event EventBeginPlay
  (bind _asmy_game_instance (Utilities|Casting|CastToMyGameInstance (Game|GetGameInstance)))
  (Variables|Default|SetMyGameInstance _asmy_game_instance)
  (bind _asbp_target_system (Utilities|Casting|CastToBP_Target_System (Variables|/Script/Engine.ChildActorComponent|GetChildActor (Variables|Default|GetTargetArrow))))
  (Variables|Default|SetTargetSystem _asbp_target_system))

(fn ConstructionScript
  (bind _cc_0 (Variables|Default|GetCC_0))
  (Transformation|SetWorldTransform _cc_0 (Math|Transform|MakeTransform (.location (Spline|GetTransformatSplinePoint (Variables|Default|GetSpline_0) 0 "World" false)) (Transformation|GetWorldRotation _cc_0) "1,1,1") false false)
  (Transformation|SetWorldRotation _cc_0 (Math|Rotator|FindLookatRotation (Transformation|GetWorldLocation _cc_0) (Transformation|GetWorldLocation (Variables|Transformation|GetRootComponent))) false false))