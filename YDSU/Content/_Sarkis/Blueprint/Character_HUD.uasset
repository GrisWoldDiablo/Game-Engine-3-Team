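; Character HUD Blueprint that puts the player's character widget on screen at the start of play.
; BeginPlay caches the player controller and MyGameInstance, then creates Char_Widget owned by that controller and adds it to the viewport.
; The remaining logic is disconnected debug leftovers that printed the current character's HP for Ball, Pyramid and Fusion, so it never runs.
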(event EventBeginPlay
  (bind _asbp_my_player_controller (Utilities|Casting|CastToBP_MyPlayerController (Game|GetPlayerController 0)))
  (bind _output_get (Variables|Default|SetPlayerController _asbp_my_player_controller))
  (bind _asmy_game_instance (Utilities|Casting|CastToMyGameInstance (Game|GetGameInstance)))
  (Variables|Default|SetMyGameInstance _asmy_game_instance)
  (bind _returnvalue (UserInterface|CreateWidget "/Game/_Sarkis/Blueprint/Char_Widget.Char_Widget_C" _output_get))
  (UserInterface|Viewport|AddtoViewport _returnvalue 0))

(event Collision|EventActorBeginOverlap
  (params (OtherActor :type Actor%20Object%20Reference)))

(event EventTick
  (params (DeltaSeconds :type Float%20%28single-precision%29)))

(fn ConstructionScript)