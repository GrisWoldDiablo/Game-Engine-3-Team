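; BP_NextLevel is a level exit actor that sends the player to the next level when MyCharacter overlaps it.
; It picks the destination from a hardcoded branch chain on the current level name, running Lvl_1a, Lvl_1b, Lvl_2, Lvl_3.
; After the first two transitions are requested, it marks the level complete in MyGameInstance and stores the current level name as LevelStartPoint.
; The Lvl_2 to Lvl_3 transition skips that progress update.
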(event EventBeginPlay
  (bind _asmy_game_instance (Utilities|Casting|CastToMyGameInstance (Game|GetGameInstance)))
  (Variables|Default|SetMyGameInstance _asmy_game_instance))

(event Collision|EventActorBeginOverlap
  (params (OtherActor :type Actor%20Object%20Reference))
  (Utilities|Casting|CastToMyCharacter OtherActor)
  (bind _returnvalue (Game|GetCurrentLevelName true))
  (if (Utilities|Enum|Equal(Enum) _returnvalue "Lvl_1a")
    (Game|OpenLevel(byName) "Lvl_1b")
    (bind _asmy_game_instance (Utilities|Casting|CastToMyGameInstance (Game|GetGameInstance) :!label _label))
    (Default|SetLevelComplete _asmy_game_instance (Variables|Default|GetLevel))
    (bind _returnvalue_2 (Game|GetCurrentLevelName true))
    (Variables|/Game/_Alex/Blueprints/Utility/MyGameInstance.MyGameInstance_C|SetLevel%20Start%20Point _asmy_game_instance _returnvalue_2)
    (elif (Utilities|Enum|Equal(Enum) _returnvalue "Lvl_1b")
      (Game|OpenLevel(byName) "Lvl_2")
      (goto _label)
      (elif (Utilities|Enum|Equal(Enum) _returnvalue "Lvl_2")
        (Game|OpenLevel(byName) "Lvl_3")))))

(event EventTick
  (params (DeltaSeconds :type Float%20%28single-precision%29)))

(fn ConstructionScript)