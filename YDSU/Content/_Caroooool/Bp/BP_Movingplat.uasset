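; Moving platform actor that slides its Cube component between the actor's origin and the position of its Sphere component.
; On BeginPlay it sets the timeline's play rate from the Speed variable and starts playback.
; Each update lerps the Cube's relative location toward the Sphere's by the timeline value, without sweep, and prints that value on screen.
; The Sphere acts as the endpoint marker.
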(event EventBeginPlay
  (Components|Timeline|SetPlayRate (Variables|Default|GetTimeline_0) (Variables|Default|GetSpeed))
  (bind _movigvalue (Timeline|Timeline_0 Play)
    (:Update
      (Development|PrintString (Utilities|String|ToString(Float) _movigvalue))
      (Transformation|SetRelativeLocation (Variables|Default|GetCube) (Math|Vector|Lerp(Vector) "0, 0, 0" (.location (Transformation|GetRelativeTransform (Variables|Default|GetSphere))) _movigvalue) false false))))

(event Collision|EventActorBeginOverlap
  (params (OtherActor :type Actor%20Object%20Reference)))

(event EventTick
  (params (DeltaSeconds :type Float%20%28single-precision%29)))

(fn ConstructionScript)