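; Player controller that manages switching between the Ball, Pyramid and Fusion characters, as allowed by each level's AvailableCharacters setting.
; On BeginPlay it takes the characters from MyGameInstance, sets their visibility and possesses the starting one.
; Input swaps Ball and Pyramid or fuses and splits them via possession, hiding, camera copying and blended view targets, updating the game instance's CurrentChar.
; Tick aims particles between the pair when within fusing range.
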(event EventBeginPlay
  ;[1 1 1] Begin Play
  (Development|PrintString (Utilities|String|EnumtoString (Variables|Default|GetAvailable%20Characters)))
  ;[1 1 1] Populate MyCharacter Variables
  (bind _asmy_game_instance (Utilities|Casting|CastToMyGameInstance (Game|GetGameInstance)))
  (bind _output_get (Variables|Default|SetMyGameInstance _asmy_game_instance))
  (Variables|Default|SetCharacter%20Pyramid (Variables|/Game/_Alex/Blueprints/Utility/MyGameInstance.MyGameInstance_C|GetCharacter%20Pyramid _output_get))
  (Variables|Default|SetCharacter%20Fusion (Variables|/Game/_Alex/Blueprints/Utility/MyGameInstance.MyGameInstance_C|GetCharacter%20Fusion _output_get))
  (Variables|Default|SetCharacter%20Ball (Variables|/Game/_Alex/Blueprints/Utility/MyGameInstance.MyGameInstance_C|GetCharacter%20Ball _output_get))
  ;[1 1 1] Initialize Characters per Level specification
  (CallFunction|InitCharacters))

(event EventTick
  (params (DeltaSeconds :type Float%20%28single-precision%29))
  (bind _character_pyramid (Variables|Default|GetCharacter%20Pyramid))
  (bind _character_pyramid_2 (Variables|Default|GetCharacter%20Pyramid))
  (bind _character_ball (Variables|Default|GetCharacter%20Ball))
  (bind _particlecomponent (Variables|/Script/YDSU.MyCharacter|GetParticleComponent _character_pyramid))
  (bind _particlecomponent_2 (Variables|/Script/YDSU.MyCharacter|GetParticleComponent _character_pyramid_2))
  (bind _particlecomponent_3 (Variables|/Script/YDSU.MyCharacter|GetParticleComponent _character_ball))
  ;[0.08142 1 0] Event Tick
  ;[1 1 1] Fusable Particle Effect
  (if (Math|Boolean|ANDBoolean (not (Variables|Default|GetIs%20Fused)) (Variables|Default|GetFusable) (Utilities|Enum|Equal(Enum) (Variables|Default|GetAvailable%20Characters) "NewEnumerator4") (<= (Transformation|GetDistanceTo (Variables|Default|GetCharacter%20Pyramid) (Variables|Default|GetCharacter%20Ball)) (Variables|Default|GetFusable%20Distance)))
    (Utilities|FlowControl|Sequence
      (:then_0
        (Components|Activation|Activate _particlecomponent_2 false)
        (Transformation|SetWorldTransform _particlecomponent_2 (Class|KismetAnimationLibrary|Lookat (Transformation|GetWorldTransform _particlecomponent_2) (Transformation|GetWorldLocation _particlecomponent_3) "1.000000, 0, 0" false "0, 0,1.000000" 0.0) false false))
      (:then_1
        (Components|Activation|Activate _particlecomponent_3 false)
        (Transformation|SetWorldTransform _particlecomponent_3 (Class|KismetAnimationLibrary|Lookat (Transformation|GetWorldTransform _particlecomponent_3) (Transformation|GetWorldLocation _particlecomponent) "1.000000, 0, 0" false "0, 0,1.000000" 0.0) false false)))
    (else
      (Components|Activation|Deactivate (Variables|/Script/YDSU.MyCharacter|GetParticleComponent (Variables|Default|GetCharacter%20Ball)))
      (Components|Activation|Deactivate _particlecomponent))))

(event Input|ActionEvents|InputActionSwap
  (params (Key :type Key%20Structure))
  (bind _character_ball (Variables|Default|GetCharacter%20Ball))
  (bind _character_pyramid (Variables|Default|GetCharacter%20Pyramid))
  (bind _available_characters (Variables|Default|GetAvailable%20Characters))
  (bind _mygameinstance (Variables|Default|GetMyGameInstance))
  ;[1 1 1] Character Swap
  (:Pressed
    (if (and (not (Variables|Default|GetIs%20Fused)) (or (Utilities|Enum|Equal(Enum) _available_characters "NewEnumerator3") (Utilities|Enum|Equal(Enum) _available_characters "NewEnumerator4")))
      (if (== (Variables|Default|GetCharacter%20Current) (Variables|Default|GetCharacter%20Pyramid))
        (Game|Player|SetViewTargetwithBlend _character_ball (Variables|Default|GetCamBlendTime) "VTBlend_Cubic" 0.0 true)
        (Pawn|Possess _character_ball)
        (Pawn|SpawnDefaultController _character_pyramid)
        (bind _output_get (Variables|Default|SetCharacter%20Current _character_ball))
        (bind _output_get_2 (Variables|/Game/_Alex/Blueprints/Utility/MyGameInstance.MyGameInstance_C|SetCurrent%20Char _mygameinstance _output_get))
        (else
          (Game|Player|SetViewTargetwithBlend _character_pyramid (Variables|Default|GetCamBlendTime) "VTBlend_Cubic" 0.0 true)
          (Pawn|Possess _character_pyramid)
          (Pawn|SpawnDefaultController _character_ball)
          (bind _output_get_3 (Variables|Default|SetCharacter%20Current _character_pyramid))
          (bind _output_get_4 (Variables|/Game/_Alex/Blueprints/Utility/MyGameInstance.MyGameInstance_C|SetCurrent%20Char _mygameinstance _output_get_3)))))))

(event Input|ActionEvents|InputActionHurt
  (params (Key :type Key%20Structure))
  ;[0 0 0 1 50] Old
  ;;[1 1 1] Test Character Healths if working properly (H), All health is stored inside MyGameInstance variables. We call the variables and here
)

(event Input|ActionEvents|InputActionJoinSplit
  (params (Key :type Key%20Structure))
  (bind _character_ball (Variables|Default|GetCharacter%20Ball))
  (bind _character_pyramid (Variables|Default|GetCharacter%20Pyramid))
  (bind _character_fusion (Variables|Default|GetCharacter%20Fusion))
  (bind _character_fusion_2 (Variables|Default|GetCharacter%20Fusion))
  (bind _character_ball_2 (Variables|Default|GetCharacter%20Ball))
  (bind _character_ball_3 (Variables|Default|GetCharacter%20Ball))
  (bind _returnvalue (Transformation|GetActorLocation _character_fusion))
  ;[1 1 1] Fuse
  (:Pressed
    (Utilities|FlowControl|DoOnce false :!label _label
      (:Completed
        (if (and (not (Variables|Default|GetIs%20Fused)) (Utilities|Enum|Equal(Enum) (Variables|Default|GetAvailable%20Characters) "NewEnumerator4"))
          (if (and (Variables|Default|GetFusable) (<= (Transformation|GetDistanceTo (Variables|Default|GetCharacter%20Pyramid) _character_ball_3) (Variables|Default|GetFusable%20Distance)))
            (if (Variables|/Game/_Alex/Blueprints/Character/BP_Ball.BP_Ball_C|GetPhysicOn _character_ball_3)
              (Default|TurnPhysic _character_ball_3))
            (Pawn|Possess _character_fusion_2)
            (CallFunction|SetActorVisibility _character_fusion_2 true)
            (CallFunction|SetActorVisibility _character_ball_2 false)
            (CallFunction|SetActorVisibility (Variables|Default|GetCharacter%20Pyramid) false)
            (Variables|Default|SetIs%20Fused true)
            (Transformation|SetActorLocation _character_fusion_2 (Transformation|GetActorLocation _character_ball_2) false false)
            (CallFunction|CopyCamValues _character_ball_2 _character_fusion_2 false)
            (Game|Player|SetViewTargetwithBlend _character_fusion_2 (Variables|Default|GetCamBlendTime) "VTBlend_Cubic" 0.0 true)
            (bind _output_get (Variables|Default|SetCharacter%20Current (Variables|Default|GetCharacter%20Fusion)))
            (bind _output_get_2 (Variables|/Game/_Alex/Blueprints/Utility/MyGameInstance.MyGameInstance_C|SetCurrent%20Char (Variables|Default|GetMyGameInstance) _output_get))
            (Components|Activation|Activate (Variables|/Script/YDSU.MyCharacter|GetParticleComponent _output_get_2) false))
          (else
            ;[1 1 1] Split
            (if (Utilities|Enum|Equal(Enum) (Variables|Default|GetAvailable%20Characters) "NewEnumerator4")
              (Pawn|Possess _character_pyramid)
              (Pawn|SpawnDefaultController _character_ball)
              (bind _output_get_3 (Variables|Default|SetCharacter%20Current _character_pyramid))
              (bind _output_get_4 (Variables|/Game/_Alex/Blueprints/Utility/MyGameInstance.MyGameInstance_C|SetCurrent%20Char (Variables|Default|GetMyGameInstance) _output_get_3))
              (CallFunction|SetActorVisibility _character_pyramid true)
              (CallFunction|SetActorVisibility _character_ball true)
              (CallFunction|SetActorVisibility _character_fusion false)
              (Transformation|SetActorLocation _character_ball _returnvalue false true)
              (Transformation|SetActorLocation _character_pyramid _returnvalue false true)
              (CallFunction|CopyCamValues _character_fusion _character_ball true)
              (CallFunction|CopyCamValues _character_fusion _character_pyramid true)
              (Variables|Default|SetIs%20Fused false)
              (Game|Player|SetViewTargetwithBlend _character_pyramid (Variables|Default|GetCamBlendTime) "VTBlend_Cubic" 0.0 true)
              (Components|Activation|Deactivate (Variables|/Script/YDSU.MyCharacter|GetParticleComponent _character_fusion))
              (Effects|SpawnEmitteratLocation "/Game/_Alex/Blueprints/Character/PS_Split.PS_Split" (Transformation|GetActorLocation _output_get_4))))))))
  (:Released
    (Utilities|FlowControl|Delay 1.0)
    (goto _label Reset)))

(fn ConstructionScript)

(fn SetActorVisibility
  (params (Actor :type Actor%20Object%20Reference%20%28by%20ref%29) (Visibility :type Boolean))
  (Rendering|SetActorHiddenInGame Actor (not Visibility))
  (Collision|SetActorEnableCollision Actor Visibility)
  (Actor|Tick|SetActorTickEnabled Actor Visibility))

(fn CopyCamValues
  (params (From%20Char :type My%20Character%20Object%20Reference%20%28by%20ref%29) (To%20Char :type My%20Character%20Object%20Reference%20%28by%20ref%29) (ChangeNow :type Boolean))
  (bind _cameraboom (Variables|/Script/YDSU.MyCharacter|GetCameraBoom To%20Char))
  (bind _output_get (Variables|/Script/YDSU.MyCharacter|SetCameraRotator To%20Char (Variables|/Script/YDSU.MyCharacter|GetCameraRotator From%20Char)))
  (bind _output_get_2 (Variables|/Script/YDSU.MyCharacter|SetCameraLenght To%20Char (Variables|/Script/YDSU.MyCharacter|GetCameraLenght From%20Char)))
  (bind _output_get_3 (Variables|/Script/YDSU.MyCharacter|SetCamLagDistance To%20Char (Variables|/Script/YDSU.MyCharacter|GetCamLagDistance From%20Char)))
  (bind _output_get_4 (Variables|/Script/YDSU.MyCharacter|SetCamLagSpeed To%20Char (Variables|/Script/YDSU.MyCharacter|GetCamLagDistance From%20Char)))
  (Transformation|SetRelativeRotation _cameraboom _output_get false false)
  (Variables|/Script/Engine.SpringArmComponent|SetTargetArmLength _cameraboom _output_get_2)
  (Variables|/Script/Engine.SpringArmComponent|SetCameraLagMaxDistance _cameraboom _output_get_3)
  (Variables|/Script/Engine.SpringArmComponent|SetCameraLagSpeed _cameraboom _output_get_4))

(fn ChangeCamera
  (params (ObjectToMove :type Scene%20Component%20Object%20Reference) (TargetLocation :type Transform) (StartLocation :type Scene%20Component%20Object%20Reference))
  (Variables|Default|SetInterpTarget ObjectToMove)
  (Variables|Default|SetTargetTinterp TargetLocation)
  (Variables|Default|SetOriginCam (Transformation|GetWorldTransform StartLocation))
  (Variables|Default|SetDoInterpCam true)
  (Variables|Default|SetIsInterpolating false))

(fn DotheCameraInterpolation
  (bind _interptarget (Variables|Default|GetInterpTarget))
  (bind _targettinterp (Variables|Default|GetTargetTinterp))
  (bind _returnvalue (Transformation|GetRelativeTransform _interptarget))
  (if (Variables|Default|GetIsInterpolating)
    _
    (else
      (Transformation|SetWorldTransform (Variables|Default|GetInterpTarget) (Variables|Default|GetOriginCam) false true)
      (Variables|Default|SetIsInterpolating true)))
  (Transformation|SetRelativeTransform _interptarget (Class|KismetMathLibrary|TInterpto _returnvalue _targettinterp (Utilities|Time|GetWorldDeltaSeconds) (Variables|Default|GetInterpolationSpeed)) false false)
  (if (Class|KismetMathLibrary|NearlyEqualTransformTransform _returnvalue _targettinterp 0.1 0.01 0.01)
    (Transformation|SetRelativeTransform _interptarget _targettinterp false false)
    (Variables|Default|SetDoInterpCam false)
    (Variables|Default|SetIsInterpolating false)
    (return true)
    (else
      (return false))))

(fn InitCharacters
  (switch Utilities|FlowControl|Switch|SwitchonECharacterType (Variables|Default|GetAvailable%20Characters)
    (:NewEnumerator0
      (CallFunction|SetActorVisibility (Variables|Default|GetCharacter%20Ball) true)
      (CallFunction|SetActorVisibility (Variables|Default|GetCharacter%20Pyramid) false)
      (CallFunction|SetActorVisibility (Variables|Default|GetCharacter%20Fusion) false)
      (Pawn|Possess (Variables|Default|GetCharacter%20Ball) :!label _label))
    (:NewEnumerator1
      (CallFunction|SetActorVisibility (Variables|Default|GetCharacter%20Ball) false)
      (CallFunction|SetActorVisibility (Variables|Default|GetCharacter%20Pyramid) true)
      (CallFunction|SetActorVisibility (Variables|Default|GetCharacter%20Fusion) false)
      (Pawn|Possess (Variables|Default|GetCharacter%20Pyramid)))
    (:NewEnumerator2
      (Variables|Default|SetIs%20Fused true :!label _label_2)
      (CallFunction|SetActorVisibility (Variables|Default|GetCharacter%20Ball) false)
      (CallFunction|SetActorVisibility (Variables|Default|GetCharacter%20Pyramid) false)
      (CallFunction|SetActorVisibility (Variables|Default|GetCharacter%20Fusion) true)
      (Pawn|Possess (Variables|Default|GetCharacter%20Fusion)))
    (:NewEnumerator3
      (CallFunction|SetActorVisibility (Variables|Default|GetCharacter%20Ball) true)
      (CallFunction|SetActorVisibility (Variables|Default|GetCharacter%20Pyramid) true)
      (CallFunction|SetActorVisibility (Variables|Default|GetCharacter%20Fusion) false)
      (goto _label))
    (:NewEnumerator4
      (goto _label_2)))
  (bind _asmy_character (Utilities|Casting|CastToMyCharacter (Pawn|GetControlledPawn (Game|GetPlayerController 0))))
  ;[1 1 1] Setting Character for Game Instance.
  (bind _output_get (Variables|Default|SetCharacter%20Current _asmy_character))
  (bind _output_get_2 (Variables|/Game/_Alex/Blueprints/Utility/MyGameInstance.MyGameInstance_C|SetCurrent%20Char (Variables|Default|GetMyGameInstance) _output_get))
  (Game|Player|SetViewTargetwithBlend _output_get_2 0.0 "VTBlend_Linear" 0.0 false))