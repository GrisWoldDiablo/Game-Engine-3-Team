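; Game instance that holds character class lookup and level completion state for the game.
; Get Character Class maps a Ball, Pyramid or Fusion choice to its stored class.
; Set Level Complete takes a level enum, flags that index in the LevelPaths array, and also sets a matching boolean from Level1 to Level5, numbered by enum order rather than level name.
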(fn GetCharacterClass
  (params (Character%20Choice :type ECharacterType%20Enum :default "NewEnumerator0"))
  (switch Utilities|FlowControl|Switch|SwitchonECharacterType Character%20Choice
    (:NewEnumerator0
      (return (Variables|Default|GetClass%20Ball)))
    (:NewEnumerator1
      (return (Variables|Default|GetClass%20Pyramid)))
    (:NewEnumerator2
      (return (Variables|Default|GetClass%20Fusion)))))

(fn SetLevelComplete
  (params (Levels :type ELevels%20Enum :default "NewEnumerator0"))
  (Utilities|Array|SetArrayElem (Variables|Default|GetLevel%20Paths) (Math|Conversions|ToInteger(Byte) Levels) true)
  (switch Utilities|FlowControl|Switch|SwitchonELevels Levels
    (:NewEnumerator0
      (Variables|Default|SetLevel%201 true))
    (:NewEnumerator1
      (Variables|Default|SetLevel%202 true))
    (:NewEnumerator2
      (Variables|Default|SetLevel%203 true))
    (:NewEnumerator3
      (Variables|Default|SetLevel%204 true))
    (:NewEnumerator4
      (Variables|Default|SetLevel%205 true))))