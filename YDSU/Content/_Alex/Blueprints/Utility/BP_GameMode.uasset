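; Game mode that spawns the Pyramid, Ball and Fusion player characters and picks player starts.
; On BeginPlay it spawns each class supplied by MyGameInstance at the start named by LevelStartPoint, stores the references back on the game instance and spawns their default controllers.
; ChoosePlayerStart lazily caches the game instance and uses LevelStartPoint only in MapLevel, looking up "None" in other levels.
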(event EventBeginPlay
  ;[1 1 1] Spawn the player characters
  (bind _asmy_game_instance (Utilities|Casting|CastToMyGameInstance (Game|GetGameInstance)))
  (Utilities|FlowControl|Sequence
    (:then_0
      (bind _returnvalue (Game|SpawnActorfromClass (Default|GetCharacterClass _asmy_game_instance "NewEnumerator1") (Transformation|GetActorTransform (Class|GameModeBase|FindPlayerStart 0 (Variables|/Game/_Alex/Blueprints/Utility/MyGameInstance.MyGameInstance_C|GetLevel%20Start%20Point _asmy_game_instance))) "Undefined" 0 0))
      (bind _asbp_pyramid (Utilities|Casting|CastToBP_Pyramid _returnvalue))
      (bind _output_get (Variables|/Game/_Alex/Blueprints/Utility/MyGameInstance.MyGameInstance_C|SetCharacter%20Pyramid _asmy_game_instance _asbp_pyramid))
      (Pawn|SpawnDefaultController _output_get))
    (:then_1
      (bind _returnvalue_2 (Game|SpawnActorfromClass (Default|GetCharacterClass _asmy_game_instance "NewEnumerator0") (Transformation|GetActorTransform (Class|GameModeBase|FindPlayerStart 0 (Variables|/Game/_Alex/Blueprints/Utility/MyGameInstance.MyGameInstance_C|GetLevel%20Start%20Point _asmy_game_instance))) "Undefined" 0 0))
      (bind _asbp_ball (Utilities|Casting|CastToBP_Ball _returnvalue_2))
      (bind _output_get_2 (Variables|/Game/_Alex/Blueprints/Utility/MyGameInstance.MyGameInstance_C|SetCharacter%20Ball _asmy_game_instance _asbp_ball))
      (Pawn|SpawnDefaultController _output_get_2))
    (:then_2
      (bind _returnvalue_3 (Game|SpawnActorfromClass (Default|GetCharacterClass _asmy_game_instance "NewEnumerator2") (Transformation|GetActorTransform (Class|GameModeBase|FindPlayerStart 0 (Variables|/Game/_Alex/Blueprints/Utility/MyGameInstance.MyGameInstance_C|GetLevel%20Start%20Point _asmy_game_instance))) "Undefined" 0 0))
      (bind _asbp_fusion (Utilities|Casting|CastToBP_Fusion _returnvalue_3))
      (bind _output_get_3 (Variables|/Game/_Alex/Blueprints/Utility/MyGameInstance.MyGameInstance_C|SetCharacter%20Fusion _asmy_game_instance _asbp_fusion))
      (Pawn|SpawnDefaultController _output_get_3))))

(fn ConstructionScript)

(fn ChoosePlayerStart
  (params (Player :type Controller%20Object%20Reference))
  (Utilities|IsValid (Variables|Default|GetMyGameInstance)
    (:Is%20Valid
      _)
    (:Is%20Not%20Valid
      (bind _asmy_game_instance (Utilities|Casting|CastToMyGameInstance (Game|GetGameInstance)))
      (bind _output_get (Variables|Default|SetMyGameInstance _asmy_game_instance))))
  (bind _returnvalue (Game|GetCurrentLevelName true))
  (if (Utilities|Enum|Equal(Enum) _returnvalue "MapLevel")
    (return (Class|GameModeBase|FindPlayerStart 0 (Variables|/Game/_Alex/Blueprints/Utility/MyGameInstance.MyGameInstance_C|GetLevel%20Start%20Point _output_get)))
    (else
      (return (Class|GameModeBase|FindPlayerStart 0 "None")))))