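; BP_LoadLevelTrigger is a world map trigger that marks a level as ready to load while the player character stands in it.
; It caches MyGameInstance on BeginPlay, then on overlap by MyCharacter sets IsReadyToLoad and passes it the trigger's LevelToLoad.
; Ending the overlap clears only the ready flag, and the trigger does not perform the load itself.
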(event EventBeginPlay
  (bind _asmy_game_instance (Utilities|Casting|CastToMyGameInstance (Game|GetGameInstance)))
  (Variables|Default|SetMyGameInstance _asmy_game_instance))

(event Collision|EventActorBeginOverlap
  (params (OtherActor :type Actor%20Object%20Reference))
  (bind _mygameinstance (Variables|Default|GetMyGameInstance))
  (Utilities|Casting|CastToMyCharacter OtherActor)
  (Variables|/Game/_Alex/Blueprints/Utility/MyGameInstance.MyGameInstance_C|SetIs%20Ready%20To%20Load _mygameinstance true)
  (Variables|/Game/_Alex/Blueprints/Utility/MyGameInstance.MyGameInstance_C|SetLevel%20To%20Load _mygameinstance (Variables|Default|GetLevel%20To%20Load)))

(event Collision|EventActorEndOverlap
  (params (OtherActor :type Actor%20Object%20Reference))
  (Utilities|Casting|CastToMyCharacter OtherActor)
  (Variables|/Game/_Alex/Blueprints/Utility/MyGameInstance.MyGameInstance_C|SetIs%20Ready%20To%20Load (Variables|Default|GetMyGameInstance) false))

(fn ConstructionScript)