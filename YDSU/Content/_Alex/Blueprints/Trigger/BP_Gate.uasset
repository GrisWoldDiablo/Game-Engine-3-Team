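; BP_Gate is a gate that opens once every trigger in its Triggers list is active.
; Each Tick until activated, it checks the Active flag of those triggers and calls OpenGate when all are set.
; OpenGate plays a timeline that lerps the Gate component from zero relative location to the OpenedPoint component's location, with no logic to close it again.
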(event Custom|OpenGate
  (bind _value (Timeline|Opening%20Timeline PlayFromStart)
    (:Update
      (Transformation|SetRelativeLocation (Variables|Default|GetGate) (Math|Vector|Lerp(Vector) "0, 0, 0" (Variables|/Script/Engine.SceneComponent|GetRelativeLocation (Variables|Default|GetOpened%20Point)) _value) false false))))

(event EventBeginPlay)

(event Collision|EventActorBeginOverlap
  (params (OtherActor :type Actor%20Object%20Reference)))

(event EventTick
  (params (DeltaSeconds :type Float%20%28single-precision%29))
  (if (not (Variables|Default|GetActivated))
    (bind _array_element (Utilities|Array|ForEachLoopwithBreak (Variables|Default|GetTriggers) :!label _label)
      (:LoopBody
        (if (not (Variables|/Game/_Alex/Blueprints/Trigger/BP_GateTrigger.BP_GateTrigger_C|GetActive _array_element))
          (Variables|Default|SetActivated false)
          (goto _label Break)
          (else
            (Variables|Default|SetActivated true))))
      (:Completed
        (if (Variables|Default|GetActivated)
          (CallFunction|OpenGate))))))

(fn ConstructionScript)