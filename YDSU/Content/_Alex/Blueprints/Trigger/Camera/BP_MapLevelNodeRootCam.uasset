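; Map level node root camera that groups four child-actor camera trigger boxes (left, right, bottom, top) around a node.
; On BeginPlay it uses the left BP_CameraTriggerBox as the master, passing its pitch, yaw and camera distance along to the other three.
; It also moves each copy's CamView back by that distance and rotates its OriginPoint to match, so all four share one camera setup.
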(event EventBeginPlay
  (|CallParentFunction)
  ;[1 1 1] Copy the setting of the left camera to the others.
  (Utilities|FlowControl|Sequence
    (:then_0
      (bind _asbp_camera_trigger_box (Utilities|Casting|CastToBP_CameraTriggerBox (Variables|/Script/Engine.ChildActorComponent|GetChildActor (Variables|Default|GetLeft%20Trigger)))))
    (:then_1
      (bind _asbp_camera_trigger_box_2 (Utilities|Casting|CastToBP_CameraTriggerBox (Variables|/Script/Engine.ChildActorComponent|GetChildActor (Variables|Default|GetRight%20Trigger))))
      (bind _output_get (Variables|/Script/YDSU.CameraTriggerBox|SetPitch _asbp_camera_trigger_box_2 (Variables|/Script/YDSU.CameraTriggerBox|GetPitch _asbp_camera_trigger_box)))
      (bind _output_get_2 (Variables|/Script/YDSU.CameraTriggerBox|SetYaw _asbp_camera_trigger_box_2 (Variables|/Script/YDSU.CameraTriggerBox|GetYaw _asbp_camera_trigger_box)))
      (bind _output_get_3 (Variables|/Script/YDSU.CameraTriggerBox|SetCameraDistance _asbp_camera_trigger_box_2 (Variables|/Script/YDSU.CameraTriggerBox|GetCameraDistance _asbp_camera_trigger_box)))
      (Transformation|SetRelativeLocation (Variables|/Script/YDSU.CameraTriggerBox|GetCamView _asbp_camera_trigger_box_2) (Math|Vector|MakeVector (* (Variables|/Script/YDSU.CameraTriggerBox|GetCameraDistance _asbp_camera_trigger_box) -1.0) 0.0 0.0) false false)
      (Transformation|SetRelativeRotation (Variables|/Script/YDSU.CameraTriggerBox|GetOriginPoint _asbp_camera_trigger_box_2) (Math|Rotator|MakeRotator 0.0 (Variables|/Script/YDSU.CameraTriggerBox|GetPitch _asbp_camera_trigger_box) (Variables|/Script/YDSU.CameraTriggerBox|GetYaw _asbp_camera_trigger_box)) false false))
    (:then_2
      (bind _asbp_camera_trigger_box_3 (Utilities|Casting|CastToBP_CameraTriggerBox (Variables|/Script/Engine.ChildActorComponent|GetChildActor (Variables|Default|GetBottom%20Trigger))))
      (bind _output_get_4 (Variables|/Script/YDSU.CameraTriggerBox|SetPitch _asbp_camera_trigger_box_3 _output_get))
      (bind _output_get_5 (Variables|/Script/YDSU.CameraTriggerBox|SetYaw _asbp_camera_trigger_box_3 _output_get_2))
      (bind _output_get_6 (Variables|/Script/YDSU.CameraTriggerBox|SetCameraDistance _asbp_camera_trigger_box_3 _output_get_3))
      (Transformation|SetRelativeLocation (Variables|/Script/YDSU.CameraTriggerBox|GetCamView _asbp_camera_trigger_box_3) (Math|Vector|MakeVector (* (Variables|/Script/YDSU.CameraTriggerBox|GetCameraDistance _asbp_camera_trigger_box) -1.0) 0.0 0.0) false false)
      (Transformation|SetRelativeRotation (Variables|/Script/YDSU.CameraTriggerBox|GetOriginPoint _asbp_camera_trigger_box_3) (Math|Rotator|MakeRotator 0.0 (Variables|/Script/YDSU.CameraTriggerBox|GetPitch _asbp_camera_trigger_box) (Variables|/Script/YDSU.CameraTriggerBox|GetYaw _asbp_camera_trigger_box)) false false))
    (:then_3
      (bind _asbp_camera_trigger_box_4 (Utilities|Casting|CastToBP_CameraTriggerBox (Variables|/Script/Engine.ChildActorComponent|GetChildActor (Variables|Default|GetTop%20Trigger))))
      (Variables|/Script/YDSU.CameraTriggerBox|SetPitch _asbp_camera_trigger_box_4 _output_get_4)
      (Variables|/Script/YDSU.CameraTriggerBox|SetYaw _asbp_camera_trigger_box_4 _output_get_5)
      (Variables|/Script/YDSU.CameraTriggerBox|SetCameraDistance _asbp_camera_trigger_box_4 _output_get_6)
      (Transformation|SetRelativeLocation (Variables|/Script/YDSU.CameraTriggerBox|GetCamView _asbp_camera_trigger_box_4) (Math|Vector|MakeVector (* (Variables|/Script/YDSU.CameraTriggerBox|GetCameraDistance _asbp_camera_trigger_box) -1.0) 0.0 0.0) false false)
      (Transformation|SetRelativeRotation (Variables|/Script/YDSU.CameraTriggerBox|GetOriginPoint _asbp_camera_trigger_box_4) (Math|Rotator|MakeRotator 0.0 (Variables|/Script/YDSU.CameraTriggerBox|GetPitch _asbp_camera_trigger_box) (Variables|/Script/YDSU.CameraTriggerBox|GetYaw _asbp_camera_trigger_box)) false false))))

(event Collision|EventActorBeginOverlap
  (params (OtherActor :type Actor%20Object%20Reference))
  (|CallParentFunction OtherActor) ; This node is disabled and will not be called.\nDrag off pins to build functionality.
)

(event EventTick
  (params (DeltaSeconds :type Float%20%28single-precision%29))
  (|CallParentFunction DeltaSeconds) ; This node is disabled and will not be called.\nDrag off pins to build functionality.
)

(fn ConstructionScript
  (|CallParentFunction))