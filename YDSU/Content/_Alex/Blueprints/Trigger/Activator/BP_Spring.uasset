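; Spring activator that launches a BP_Ball along its forward vector when its linked Trigger becomes active.
; Tick polls the Trigger and latches Activated, firing the mesh once per activation through simulated physics and an impulse.
; Hitting the ball enables its physics, resets its velocity, applies a Strength-scaled impulse and stops the mesh simulation.
; After a short delay, a timeline lerps the mesh's relative location toward the actor's world location.
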(event Custom|Spring
  (bind _staticmesh (Variables|Default|GetStaticMesh))
  (Physics|SetSimulatePhysics _staticmesh true)
  (Physics|AddImpulse _staticmesh (* (Transformation|GetActorForwardVector) 1e+03) "None" true))

(event EventBeginPlay)

(event Collision|EventActorBeginOverlap
  (params (OtherActor :type Actor%20Object%20Reference)))

(event EventTick
  (params (DeltaSeconds :type Float%20%28single-precision%29))
  (bind _staticmesh (Variables|Default|GetStaticMesh))
  (bind _staticmesh_2 (Variables|Default|GetStaticMesh))
  (if (Variables|/Game/_Alex/Blueprints/Trigger/Activator/BP_ActivatorTrigger.BP_ActivatorTrigger_C|GetActive (Variables|Default|GetTrigger))
    (if (not (stale _output_get))
      (Development|PrintString "Spring")
      (Variables|Default|SetActivated true)
      (CallFunction|Spring)
      (Utilities|FlowControl|Delay 0.5)
      (Class|PrimitiveComponent|SetAllPhysicsLinearVelocity _staticmesh_2 "0, 0, 0" false)
      (Physics|SetSimulatePhysics _staticmesh_2 false)
      (bind _value (Timeline|Timeline_0 PlayFromStart)
        (:Update
          (Transformation|SetRelativeLocation _staticmesh (Math|Vector|Lerp(Vector) (Variables|/Script/Engine.SceneComponent|GetRelativeLocation _staticmesh) (Transformation|GetActorLocation) _value) false false))))
    (else
      (bind _output_get (Variables|Default|SetActivated false)))))

(event Collision|EventHit
  (params (MyComp :type Primitive%20Component%20Object%20Reference) (Other :type Actor%20Object%20Reference) (OtherComp :type Primitive%20Component%20Object%20Reference) (bSelfMoved :type Boolean) (HitLocation :type Vector :default "0, 0, 0") (HitNormal :type Vector :default "0, 0, 0") (NormalImpulse :type Vector :default "0, 0, 0") (Hit :type Hit%20Result%20Structure%20%28by%20ref%29))
  (if (Class|SceneComponent|IsAnySimulatingPhysics (Variables|Default|GetStaticMesh))
    (Development|PrintString "Hit!")
    (bind _asbp_ball (Utilities|Casting|CastToBP_Ball Other))
    (if (not (Variables|/Game/_Alex/Blueprints/Character/BP_Ball.BP_Ball_C|GetPhysicOn _asbp_ball))
      (Default|TurnPhysic _asbp_ball))
    (Class|PrimitiveComponent|SetAllPhysicsLinearVelocity (Variables|/Script/Engine.Character|GetCapsuleComponent _asbp_ball) "0, 0, 0" false)
    (Physics|AddImpulse (Variables|/Script/Engine.Character|GetCapsuleComponent _asbp_ball) (* (Transformation|GetActorForwardVector) (Variables|Default|GetStrength)) "None" true)
    (Physics|SetSimulatePhysics (Variables|Default|GetStaticMesh) false)))

(fn ConstructionScript)