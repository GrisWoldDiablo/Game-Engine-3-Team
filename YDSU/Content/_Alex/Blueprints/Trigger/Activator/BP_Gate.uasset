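; BP_Gate is a gate or platform that moves linearly or rotates in response to an array of triggers.
; Tick checks triggers by GateType: AND types open once and stay open, while OR types open or reclose as triggers change.
; One timeline, rate set by MovementSpeed, lerps the mesh location or pivot rotation toward values from reference components.
; An OverrideActivate flag forces it open.
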(event Custom|OpenGate
  ;[1 1 1] Single activation
  (bind _value (Timeline|Opening%20Timeline PlayFromStart)
    (:Update
      ;[1 1 1] Gate type choice
      (switch Utilities|FlowControl|Switch|SwitchonEGateType (Variables|Default|GetGate%20Type)
        (:NewEnumerator0
          ;[1 1 1] Linear Movement
          (Transformation|SetRelativeLocation (Variables|Default|GetGate/Bridge/Platform%20Mesh) (Math|Vector|Lerp(Vector) "0, 0, 0" (Variables|/Script/Engine.SceneComponent|GetRelativeLocation (Variables|Default|GetOpened%20Location)) _value) false false :!label _label))
        (:NewEnumerator1
          (goto _label))
        (:NewEnumerator3
          ;[1 1 1] Rotation movement
          (Transformation|SetRelativeRotation (Variables|Default|GetRotation%20Point) (Math|Rotator|Lerp(Rotator) "0, 0, 0" (Variables|/Script/Engine.SceneComponent|GetRelativeRotation (Variables|Default|GetRotation%20Value)) _value) false false :!label _label_2))
        (:NewEnumerator4
          (goto _label_2))))))

(event Custom|Cycle%20Open%20Gate
  ;[1 1 1] Hold activation
  (bind _value (Timeline|Opening%20Timeline Play)
    (:Update
      ;[1 1 1] Gate type choice
      (switch Utilities|FlowControl|Switch|SwitchonEGateType (Variables|Default|GetGate%20Type)
        (:NewEnumerator0
          ;[1 1 1] Linear Movement
          (Transformation|SetRelativeLocation (Variables|Default|GetGate/Bridge/Platform%20Mesh) (Math|Vector|Lerp(Vector) "0, 0, 0" (Variables|/Script/Engine.SceneComponent|GetRelativeLocation (Variables|Default|GetOpened%20Location)) _value) false false :!label _label))
        (:NewEnumerator1
          (goto _label))
        (:NewEnumerator3
          ;[1 1 1] Rotation movement
          (Transformation|SetRelativeRotation (Variables|Default|GetRotation%20Point) (Math|Rotator|Lerp(Rotator) "0, 0, 0" (Variables|/Script/Engine.SceneComponent|GetRelativeRotation (Variables|Default|GetRotation%20Value)) _value) false false :!label _label_2))
        (:NewEnumerator4
          (goto _label_2))))))

(event Custom|Cycle%20Close%20Gate
  ;[1 1 1] Hold activation
  (bind _value (Timeline|Opening%20Timeline Reverse)
    (:Update
      ;[1 1 1] Gate type choice
      (switch Utilities|FlowControl|Switch|SwitchonEGateType (Variables|Default|GetGate%20Type)
        (:NewEnumerator0
          ;[1 1 1] Linear Movement
          (Transformation|SetRelativeLocation (Variables|Default|GetGate/Bridge/Platform%20Mesh) (Math|Vector|Lerp(Vector) "0, 0, 0" (Variables|/Script/Engine.SceneComponent|GetRelativeLocation (Variables|Default|GetOpened%20Location)) _value) false false :!label _label))
        (:NewEnumerator1
          (goto _label))
        (:NewEnumerator3
          ;[1 1 1] Rotation movement
          (Transformation|SetRelativeRotation (Variables|Default|GetRotation%20Point) (Math|Rotator|Lerp(Rotator) "0, 0, 0" (Variables|/Script/Engine.SceneComponent|GetRelativeRotation (Variables|Default|GetRotation%20Value)) _value) false false :!label _label_2))
        (:NewEnumerator4
          (goto _label_2))))))

(event EventBeginPlay
  ;[1 1 1] Set Movement speed
  (Components|Timeline|SetPlayRate (Variables|Default|GetOpening%20Timeline) (Variables|Default|GetMovement%20Speed)))

(event EventTick
  (params (DeltaSeconds :type Float%20%28single-precision%29))
  (if (Variables|Default|GetOverride%20Activate)
    (CallFunction|OpenGate)
    (Variables|Default|SetActivated true)
    (Variables|Default|SetOverride%20Activate false)
    (else
      ;[1 1 1] Gate type choice
      (switch Utilities|FlowControl|Switch|SwitchonEGateType (Variables|Default|GetGate%20Type)
        (:NewEnumerator0
          ;[1 1 1] Stays open once activated trigger.
          (if (not (Variables|Default|GetActivated)) :!label _label
            (bind _array_element (Utilities|Array|ForEachLoopwithBreak (Variables|Default|GetTriggers) :!label _label_2)
              (:LoopBody
                (if (not (Variables|/Game/_Alex/Blueprints/Trigger/Activator/BP_ActivatorTrigger.BP_ActivatorTrigger_C|GetActive _array_element))
                  (Variables|Default|SetActivated false)
                  (goto _label_2 Break)
                  (else
                    (Variables|Default|SetActivated true))))
              (:Completed
                (if (Variables|Default|GetActivated)
                  (CallFunction|OpenGate))))))
        (:NewEnumerator1
          ;[1 1 1] Stays open on trigger hold
          (bind _array_element_2 (Utilities|Array|ForEachLoopwithBreak (Variables|Default|GetTriggers) :!label _label_3)
            (:LoopBody
              (if (Variables|/Game/_Alex/Blueprints/Trigger/Activator/BP_ActivatorTrigger.BP_ActivatorTrigger_C|GetActive _array_element_2)
                (Variables|Default|SetCan%20Cycle true)
                (goto _label_3 Break)
                (else
                  (Variables|Default|SetCan%20Cycle false))))
            (:Completed
              (if (Variables|Default|GetCan%20Cycle)
                (CallFunction|CycleOpenGate)
                (else
                  (CallFunction|CycleCloseGate))))))
        (:NewEnumerator3
          (goto _label))
        (:NewEnumerator4
          (goto _label_3))))))

(fn ConstructionScript)