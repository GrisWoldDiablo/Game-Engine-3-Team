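; Game mode Blueprint that decides where the player spawns in each level.
; Its ChoosePlayerStart override checks whether the current level is MapLevel and, if so, passes LastLevel from MyGameInstance to FindPlayerStart as the start name, so the spawn point follows the last recorded level.
; Other levels look up the start with the name "None", and the event graph is empty.
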(event EventBeginPlay)

(event EventTick
  (params (DeltaSeconds :type Float%20%28single-precision%29)))

(fn ConstructionScript)

(fn ChoosePlayerStart
  (params (Player :type Controller%20Object%20Reference))
  (bind _returnvalue (Game|GetCurrentLevelName true))
  (if (Utilities|Enum|Equal(Enum) _returnvalue "MapLevel")
    (bind _asmy_game_instance (Utilities|Casting|CastToMyGameInstance (Game|GetGameInstance)))
    (return (Class|GameModeBase|FindPlayerStart Player (Utilities|String|ToString(Name) (Variables|/Game/_Alex/Blueprints/MyGameInstance.MyGameInstance_C|GetLast%20Level _asmy_game_instance))))
    (else
      (return (Class|GameModeBase|FindPlayerStart Player "None")))))