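; Behavior tree task that makes a BP_CubeEnemy play a melee attack montage against the Player stored in its blackboard.
; A random roll picks the common kick or the rarer punch, sets an Attacking flag until the montage completes, and finishes the task without waiting for it.
; A hidden player is cleared from the blackboard instead.
; While Attacking is set, execution does nothing and never calls finish.
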(event EventReceiveExecuteAI
  (params (OwnerController :type AI%20Controller%20Object%20Reference) (ControlledPawn :type Pawn%20Object%20Reference))
  (bind _returnvalue (Utilities|Name|MakeLiteralName "Player"))
  (bind _returnvalue_2 (AI|GetBlackboard ControlledPawn))
  (bind _asbp_cube_enemy (Utilities|Casting|CastToBP_CubeEnemy ControlledPawn))
  (if (not (Variables|Default|GetAttacking))
    (bind _asmy_character (Utilities|Casting|CastToMyCharacter (AI|Components|Blackboard|GetValueasObject (AI|GetBlackboard ControlledPawn) _returnvalue)))
    (if (not (Variables|/Script/Engine.Actor|GetbHidden _asmy_character))
      (Math|Float|CompareFloat (Math|Random|RandomFloat) 0.8
        (:>
          (Animation|Montage|PlayMontage (Variables|/Script/Engine.Character|GetMesh _asbp_cube_enemy) "/Game/_Alex/Animations/Enemies/Cube/Attack/AM_Punch.AM_Punch" :!label _label
            (:then
              (Variables|Default|SetAttacking true :!label _label_2))
            (:OnCompleted
              (Variables|Default|SetAttacking false :!label _label_3))))
        (:==
          (goto _label))
        (:<
          (Animation|Montage|PlayMontage (Variables|/Script/Engine.Character|GetMesh _asbp_cube_enemy) "/Game/_Alex/Animations/Enemies/Cube/Attack/AM_Kick.AM_Kick"
            (:then
              (goto _label_2))
            (:OnCompleted
              (goto _label_3)))))
      (AI|BehaviorTree|FinishExecute true)
      (else
        (AI|Components|Blackboard|SetValueasObject _returnvalue_2 _returnvalue 0)
        (Development|PrintString (Utilities|String|Append "Untargeting: " (Utilities|GetDisplayName (AI|Components|Blackboard|GetValueasObject _returnvalue_2 _returnvalue))))
        (AI|BehaviorTree|FinishExecute true)))))