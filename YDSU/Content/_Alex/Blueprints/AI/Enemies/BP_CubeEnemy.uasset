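; Cube enemy character driven by an AI blackboard, with kick and punch hitbox attacks and a projectile throw aimed at the player.
; Damage lowers HP, which feeds the target arrow shown while it is targeted; death plays a montage, unpossesses it and rolls a pickup drop.
; A targeted kill triggers a finisher: per-actor time dilation and a spline-driven camera orienting toward the spline, then view and input return.
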(event Custom|Throw
  (bind _projectilespawn (Variables|Default|GetProjectileSpawn))
  (bind _returnvalue (Transformation|GetWorldTransform _projectilespawn))
  ;[0.5172 1 0.1739] Throw Attack
  (bind _asmy_character (Utilities|Casting|CastToMyCharacter (AI|Components|Blackboard|GetValueasObject (AI|GetBlackboard 0) (Utilities|Name|MakeLiteralName "Player"))))
  (Transformation|SetWorldTransform _projectilespawn (Class|KismetAnimationLibrary|Lookat (Transformation|GetWorldTransform _projectilespawn) (Transformation|GetActorLocation _asmy_character) "1.000000, 0,0.000000" false "0, 0,1.000000" 0.0) false true)
  (bind _returnvalue_2 (Game|SpawnActorfromClass "/Game/_Alex/Blueprints/AI/Enemies/BP_CubeProjectile.BP_CubeProjectile_C" (Math|Transform|MakeTransform (.location _returnvalue) (.rotation _returnvalue) "1,1,1") "Undefined" 0 0))
  (Variables|/Script/YDSU.CubeProjectile|SetDamage _returnvalue_2 (Variables|Default|GetDamage)))

(event Custom|FInisherCam
  (bind _spline (Variables|Default|GetSpline))
  (bind _cc (Variables|Default|GetCC))
  ;[1 0.8337 0] Finisher Camera
  (Pawn|Components|CharacterMovement|DisableMovement (Variables|Character|GetCharacterMovement))
  (bind _track_percentage (Timeline|Camera%20Timeline Play)
    (:Update
      (Transformation|SetWorldTransform _cc (Math|Transform|MakeTransform (.location (Spline|GetTransformatDistanceAlongSpline _spline (* _track_percentage (Spline|GetSplineLength _spline)) "World" false)) (Math|Rotator|FindLookatRotation (Transformation|GetWorldLocation _cc) (Transformation|GetWorldLocation (Variables|Default|GetSpline))) (.scale (Spline|GetTransformatDistanceAlongSpline _spline (* _track_percentage (Spline|GetSplineLength _spline)) "World" false))) false false))
    (:Finished
      (CallFunction|ResetCam))))

(event Custom|Punch
  (bind _hit_area (Variables|Default|GetHit%20Area))
  ;[0.5172 1 0.1739] Kick or Punch Attack
  (Collision|SetCollisionEnabled _hit_area "QueryOnly")
  (for _array_element (Collision|GetOverlappingActors _hit_area "/Script/YDSU.MyCharacter" :!class /Script/Engine.PrimitiveComponent)
    (bind _asmy_character (Utilities|Casting|CastToMyCharacter _array_element))
    (Game|Damage|ApplyDamage _asmy_character (Math|Conversions|ToFloat(Integer) (Variables|Default|GetDamage)) 0 0)
    (Collision|SetCollisionEnabled (Variables|Default|GetHit%20Area) "NoCollision"))
  (Collision|SetCollisionEnabled (Variables|Default|GetHit%20Area) "NoCollision"))

(event Custom|Kick
  (bind _hit_area (Variables|Default|GetHit%20Area))
  ;[0.5172 1 0.1739] Kick or Punch Attack
  (Collision|SetCollisionEnabled _hit_area "QueryOnly")
  (for _array_element (Collision|GetOverlappingActors _hit_area "/Script/YDSU.MyCharacter" :!class /Script/Engine.PrimitiveComponent)
    (bind _asmy_character (Utilities|Casting|CastToMyCharacter _array_element))
    (Game|Damage|ApplyDamage _asmy_character (Math|Conversions|ToFloat(Integer) (Variables|Default|GetDamage)) 0 0)
    (Collision|SetCollisionEnabled (Variables|Default|GetHit%20Area) "NoCollision"))
  (Collision|SetCollisionEnabled (Variables|Default|GetHit%20Area) "NoCollision"))

(event Custom|ResetCam
  ;[1 0.8337 0] Return camera to Player and reset time dilation.
  (Game|Player|SetViewTargetwithBlend (Variables|Default|GetMyPlayerController) (Variables|/Game/_Alex/Blueprints/Utility/MyGameInstance.MyGameInstance_C|GetCurrent%20Char (Variables|Default|GetMyGameInstance)) (Variables|Default|GetFinisher%20Cam%20Time) "VTBlend_Linear" 0.0 false)
  (Utilities|FlowControl|Delay (Variables|Default|GetFinisher%20Cam%20Time))
  (for _array_element (stale Game|Damage|EventAnyDamage _outactors)
    (Utilities|IsValid _array_element
      (:Is%20Valid
        (Variables|/Script/Engine.Actor|SetCustomTimeDilation _array_element 1.0)
        (Input|EnableInput (Variables|/Game/_Alex/Blueprints/Utility/MyGameInstance.MyGameInstance_C|GetCurrent%20Char (Variables|Default|GetMyGameInstance)) (Variables|Default|GetMyPlayerController))))))

(event EventBeginPlay
  ;[1 0 0.9142] Begin Play
  (bind _asmy_game_instance (Utilities|Casting|CastToMyGameInstance (Game|GetGameInstance)))
  (Variables|Default|SetMyGameInstance _asmy_game_instance)
  (bind _asbp_target_system (Utilities|Casting|CastToBP_Target_System (Variables|/Script/Engine.ChildActorComponent|GetChildActor (Variables|Default|GetTarget%20Arrow))))
  (Variables|Default|SetTargetSystem _asbp_target_system)
  (bind _asbp_my_player_controller (Utilities|Casting|CastToBP_MyPlayerController (Game|GetPlayerController 0)))
  (Variables|Default|SetMyPlayerController _asbp_my_player_controller)
  (AI|Components|Blackboard|SetValueasBool (AI|GetBlackboard 0) (Utilities|Name|MakeLiteralName "Range") (Variables|Default|GetRange)))

(event EventTick
  (params (DeltaSeconds :type Float%20%28single-precision%29))
  (bind _target_arrow (Variables|Default|GetTarget%20Arrow))
  ;[1 1 1] Set the Target arrow On or Off adjust the Color value
  (Variables|/Game/_Sarkis/Blueprint/BP_Target_System.BP_Target_System_C|Settest (Variables|Default|GetTargetSystem) (/ (Math|Conversions|ToFloat(Integer) (Variables|Default|GetHP)) (Math|Conversions|ToFloat(Integer) (Variables|Default|GetMaxHP))))
  (if (== (Variables|/Game/_Alex/Blueprints/Utility/MyGameInstance.MyGameInstance_C|GetEnemy%20Targeted (Variables|Default|GetMyGameInstance)) self)
    (Rendering|SetVisibility _target_arrow true false)
    (else
      (Rendering|SetVisibility _target_arrow false false))))

(event Game|Damage|EventAnyDamage
  (params (Damage :type Float%20%28single-precision%29) (DamageType :type Damage%20Type%20Object%20Reference) (InstigatedBy :type Controller%20Object%20Reference) (DamageCauser :type Actor%20Object%20Reference))
  (bind _mygameinstance (Variables|Default|GetMyGameInstance))
  (bind _pickup_choices (Variables|Default|GetPickup%20Choices))
  ;[1 0.4973 0.5471] Receiving Damage
  (bind _damage_out (CallFunction|TakeDamage Damage))
  (bind _output_get (Variables|Default|SetHP (- (Variables|Default|GetHP) (Math|Float|Truncate _damage_out))))
  ;[0.3542 0.03157 0] Dying
  (Math|Integer|CompareInt _output_get
    (:==
      _)
    (:<
      _))
  ;;[1 0.8337 0] If targeted call finisher camera
  (if (== self (Variables|/Game/_Alex/Blueprints/Utility/MyGameInstance.MyGameInstance_C|GetEnemy%20Targeted _mygameinstance))
    (Utilities|FlowControl|Sequence
      (:then_0
        ;[1 0.8337 0] Set the proper bullet time effect to all actors and call finisher camera
        (bind _outactors (Actor|GetAllActorsOfClass "/Script/Engine.Actor"))
        (for _array_element _outactors
          (Utilities|Casting|CastToMyCharacter _array_element
            (:CastFailed
              (Variables|/Script/Engine.Actor|SetCustomTimeDilation _array_element 0.0))))
        (Variables|Default|SetCustomTimeDilation 0.2)
        (Game|Player|SetViewTargetwithBlend (Variables|Default|GetMyPlayerController) self (Variables|Default|GetFinisher%20Cam%20Time) "VTBlend_Linear" 0.0 false)
        (Input|DisableInput (Variables|/Game/_Alex/Blueprints/Utility/MyGameInstance.MyGameInstance_C|GetCurrent%20Char (Variables|Default|GetMyGameInstance)) (Variables|Default|GetMyPlayerController))
        (Utilities|FlowControl|Delay (Variables|Default|GetFinisher%20Cam%20Time))
        (CallFunction|FInisherCam))
      (:then_1
        (Variables|/Game/_Alex/Blueprints/Utility/MyGameInstance.MyGameInstance_C|SetEnemy%20Targeted _mygameinstance 0)
        (Utilities|Array|RemoveItem (Variables|/Game/_Alex/Blueprints/Utility/MyGameInstance.MyGameInstance_C|GetEnemies%20In%20Range _mygameinstance) self :!label _label)
        (Animation|Montage|PlayMontage (Variables|Character|GetMesh) "/Game/_Alex/Animations/Enemies/Cube/Misc/AM_Die.AM_Die"
          (:then
            (Pawn|UnPossess (AI|GetAIController self))
            (Collision|SetActorEnableCollision false)
            (bind _asbp_fusion (Utilities|Casting|CastToBP_Fusion (Variables|/Game/_Alex/Blueprints/Utility/MyGameInstance.MyGameInstance_C|GetCurrent%20Char (Variables|Default|GetMyGameInstance))))
            (Variables|/Game/_Alex/Blueprints/Character/BP_Fusion.BP_Fusion_C|SetIsTargeting _asbp_fusion false)
            ;;[0.2456 1 0.3141] Drop Pickup
            (Utilities|FlowControl|Delay 2.0)
            (Math|Float|CompareFloat (Math|Random|RandomFloat) (Variables|Default|GetPickup%20Drop%20Rate)
              (:==
                _)
              (:<
                _))
            (Game|SpawnActorfromClass (Utilities|Array|Get(acopy) _pickup_choices (Math|Random|RandomIntegerinRange 0 (Utilities|Array|LastIndex _pickup_choices))) (Transformation|GetActorTransform) "Undefined" 0 0)))))
    (else
      (goto _label))))

(fn ConstructionScript
  (bind _cc (Variables|Default|GetCC))
  (Transformation|SetWorldTransform _cc (Math|Transform|MakeTransform (.location (Spline|GetTransformatSplinePoint (Variables|Default|GetSpline) 0 "World" false)) (Transformation|GetWorldRotation _cc) "1,1,1") false false)
  (Transformation|SetWorldRotation _cc (Math|Rotator|FindLookatRotation (Transformation|GetWorldLocation _cc) (Transformation|GetWorldLocation (Variables|Transformation|GetRootComponent))) false false))

(fn TakeDamage
  (params (Damage%20In :type Float%20%28single-precision%29))
  (return Damage%20In))