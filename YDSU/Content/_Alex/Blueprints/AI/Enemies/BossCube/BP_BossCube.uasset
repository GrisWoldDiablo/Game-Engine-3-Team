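; Cube boss enemy that drives its phases (wander, attack, shelter, run) through its AI controller and Blackboard.
; Tick checks health in each attack phase to trigger shelters that spawn BossMechanic waves, or, in the first, a fast retreat that ends with full healing.
; Damage is reduced by armor and nullified while the Sheltering flag is set.
; A charged ground pound launches and damages nearby players, with particle effects.
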(event Custom|EndShelter2
  ;[1 1 1] End Shelter
  (Animation|Montage|PlayMontage (Variables|Character|GetMesh) "/Game/_Alex/Animations/Enemies/Cube/Power/AM_ShelterOut.AM_ShelterOut"
    (:OnCompleted
      (CallFunction|ShelterOut "NewEnumerator2"))))

(event Custom|Destroy%20Charge
  ;[0.5172 1 0.1739] Ground Pound
  (Components|DestroyComponent (Variables|Default|GetParticle%20Ground%20Pound)))

(event Custom|EndShelter1
  ;[1 1 1] End Shelter
  (Animation|Montage|PlayMontage (Variables|Character|GetMesh) "/Game/_Alex/Animations/Enemies/Cube/Power/AM_ShelterOut.AM_ShelterOut"
    (:OnCompleted
      (CallFunction|ShelterOut "NewEnumerator0"))))

(event EventBeginPlay
  ;[1 0 0.9142] Begin Play
  (|CallParentFunction)
  (bind _asaic_boss_cube (Utilities|Casting|CastToAIC_BossCube (AI|GetAIController self)))
  (Variables|Default|SetAIC%20Boss _asaic_boss_cube)
  (CallFunction|ChangePhase "NewEnumerator4"))

(event EventTick
  (params (DeltaSeconds :type Float%20%28single-precision%29))
  (bind _returnvalue (|HPPercentage))
  (|CallParentFunction DeltaSeconds)
  (switch Utilities|FlowControl|Switch|SwitchonEBossPhase (Variables|/Game/_Alex/Blueprints/AI/Enemies/BossCube/AIC_BossCube.AIC_BossCube_C|GetPhase (Variables|Default|GetAIC%20Boss))
    (:NewEnumerator0
      (Math|Float|CompareFloat _returnvalue 0.6
        (:==
          _)
        (:<
          _))
      (Math|Float|CompareFloat _returnvalue 0.4
        (:>
          (if (not (Variables|Default|GetSheltering))
            (Utilities|FlowControl|DoOnce false
              (:Completed
                (CallFunction|Shelterin "NewEnumerator1")
                (Utilities|FlowControl|Delay 1.0)
                (Default|SpawnFirstWave (Variables|Default|GetBoss%20Mechanic))))))
        (:==
          (CallFunction|Run :!label _label))
        (:<
          (goto _label))))
    (:NewEnumerator2
      (Math|Float|CompareFloat (|HPPercentage_2) 0.6
        (:==
          _)
        (:<
          _))
      (Utilities|FlowControl|DoOnce false
        (:Completed
          (CallFunction|Shelterin "NewEnumerator5")
          (Utilities|FlowControl|Delay 1.0)
          (Default|SpawnSecondWave (Variables|Default|GetBoss%20Mechanic)))))))

(event EventGroundPound
  ;[0.5172 1 0.1739] Ground Pound
  (Utilities|FlowControl|Sequence
    (:then_0
      (Effects|SpawnEmitteratLocation "/Game/_Alex/Blueprints/AI/Enemies/BossCube/PS_GroundPoundExplosion.PS_GroundPoundExplosion" (Transformation|GetWorldLocation (stale EventGroundPoundCharge _output_get))))
    (:then_1
      (CallFunction|DestroyCharge)
      (bind _outactors (Collision|SphereOverlapActors (Transformation|GetActorLocation) 5e+02 (Utilities|Array|MakeArray "ObjectTypeQuery3") "/Script/YDSU.MyCharacter" (Utilities|Array|MakeArray 0)))
      (for _array_element _outactors
        (bind _asmy_character (Utilities|Casting|CastToMyCharacter _array_element))
        (Character|LaunchCharacter _asmy_character (* (+ (* (Transformation|GetActorUpVector _asmy_character) 2.0) (Math|Vector|GetUnitDirection(Vector) (Transformation|GetActorLocation) (Transformation|GetActorLocation _asmy_character))) (Variables|Default|GetGround%20Pound%20Force)) false false)
        (Game|Damage|ApplyDamage _asmy_character (* (Variables|Default|GetDamage) 3.0) 0 0)
        (Effects|SpawnEmitterAttached "/Game/_Alex/Blueprints/AI/Enemies/BossCube/PS_GroundPoundTouch.PS_GroundPoundTouch" (Variables|/Script/Engine.Character|GetCapsuleComponent _asmy_character) "None" "0, 0, 0" "0, 0, 0" "1.000000,1.000000,1.000000" "SnapToTarget")))))

(event EventGroundPoundCharge
  ;[0.5172 1 0.1739] Ground Pound
  (bind _returnvalue (Effects|SpawnEmitteratLocation "/Game/_Alex/Blueprints/AI/Enemies/BossCube/PS_GroundPoundCharge.PS_GroundPoundCharge" (Transformation|GetWorldLocation (Variables|Character|GetMesh))))
  (bind _output_get (Variables|Default|SetParticle%20Ground%20Pound _returnvalue)))

(fn ConstructionScript
  (|CallParentFunction))

(fn TakeDamage
  (params (Damage%20In :type Float%20%28single-precision%29))
  (if (not (Variables|Default|GetSheltering))
    (bind _damage_out (|CallParentFunction (/ Damage%20In (Variables|Default|GetArmor))))
    (return _damage_out)
    (else
      (bind _damage_out_2 (|CallParentFunction 0.0))
      (return _damage_out_2))))

(fn Shelterin
  (params (Phase :type EBossPhase%20Enum :default "NewEnumerator0"))
  (CallFunction|ChangePhase Phase)
  (bind _returnvalue (Effects|SpawnEmitteratLocation "/Game/_Alex/Blueprints/AI/Enemies/BossCube/PS_Shelter.PS_Shelter" (Transformation|GetWorldLocation (Variables|Character|GetMesh))))
  (Variables|Default|SetParticle%20Shelter _returnvalue)
  (Pawn|Components|CharacterMovement|DisableMovement (Variables|Character|GetCharacterMovement)))

(fn ShelterOut
  (params (NewParam :type EBossPhase%20Enum :default "NewEnumerator0"))
  (CallFunction|ChangePhase NewParam)
  (Variables|Default|SetSheltering false)
  (Components|DestroyComponent (Variables|Default|GetParticle%20Shelter))
  (Effects|SpawnEmitteratLocation "/Game/_Alex/Blueprints/AI/Enemies/BossCube/PS_ShelterOut.PS_ShelterOut" (Transformation|GetWorldLocation (Variables|Character|GetMesh)))
  (Pawn|Components|CharacterMovement|SetMovementMode (Variables|Character|GetCharacterMovement) "MOVE_Walking" 0))

(fn Run
  (bind _charactermovement (Variables|Character|GetCharacterMovement))
  (Variables|Default|SetSheltering true)
  (CallFunction|ChangePhase "NewEnumerator3")
  (AI|Components|Blackboard|SetValueasVector (Variables|/Script/AIModule.AIController|GetBlackboard (Variables|Default|GetAIC%20Boss)) (Utilities|Name|MakeLiteralName "MoveToLocation") (Variables|/Game/_Alex/Blueprints/AI/Enemies/BossCube/BP_BossMechanic.BP_BossMechanic_C|GetRun%20Location (Variables|Default|GetBoss%20Mechanic)))
  (Variables|/Script/Engine.CharacterMovementComponent|SetMaxWalkSpeed _charactermovement (* (Variables|/Script/Engine.CharacterMovementComponent|GetMaxWalkSpeed _charactermovement) 2.0))
  (Collision|SetCollisionResponsetoChannel (Variables|Default|GetCapsuleComponent) "ECC_Pawn" "ECR_Ignore"))

(fn ChangePhase
  (params (Phase :type EBossPhase%20Enum :default "NewEnumerator0"))
  (bind _aic_boss (Variables|Default|GetAIC%20Boss))
  (bind _output_get (Variables|/Game/_Alex/Blueprints/AI/Enemies/BossCube/AIC_BossCube.AIC_BossCube_C|SetPhase _aic_boss Phase))
  (AI|Components|Blackboard|SetValueasEnum (Variables|/Script/AIModule.AIController|GetBlackboard _aic_boss) (Utilities|Name|MakeLiteralName "Phase") _output_get))

(fn StopRunning
  (bind _charactermovement (Variables|Character|GetCharacterMovement))
  (Variables|Default|SetSheltering false)
  (Variables|Default|SetHP (Variables|Default|GetMaxHP))
  (Variables|/Script/Engine.CharacterMovementComponent|SetMaxWalkSpeed _charactermovement (/ (Variables|/Script/Engine.CharacterMovementComponent|GetMaxWalkSpeed _charactermovement) 2.0))
  (CallFunction|ChangePhase "NewEnumerator4")
  (Collision|SetCollisionResponsetoChannel (Variables|Default|GetCapsuleComponent) "ECC_Pawn" "ECR_Block"))

(fn SetPlayer
  (params (Player :type My%20Character%20Object%20Reference))
  (AI|Components|Blackboard|SetValueasObject (Variables|/Script/AIModule.AIController|GetBlackboard (Variables|Default|GetAIC%20Boss)) (Utilities|Name|MakeLiteralName "Player") Player))