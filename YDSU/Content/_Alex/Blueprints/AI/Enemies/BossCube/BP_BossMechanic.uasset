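; Level actor that runs the BossCube fight's encounter mechanics: enemy waves, gates, platforms and the death reward.
; Tick polls the boss AI phase, opening the first gate in Run and ending each Shelter phase once all spawned enemies have lost their AI controllers.
; Wave functions spawn enemies at placed markers; the second adds ranged enemies and activates phase-two platforms.
; Boss death reveals objects hidden at BeginPlay and briefly shows a death widget.
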(event EventBeginPlay
  (bind _asmy_game_instance (Utilities|Casting|CastToMyGameInstance (Game|GetGameInstance)))
  (Variables|Default|SetGame%20Instance _asmy_game_instance)
  (for _array_element (Variables|Default|GetDead%20Boss%20Spawn%20Object)
    (CallFunction|SetActorVisibility _array_element false)))

(event Collision|EventActorBeginOverlap
  (params (OtherActor :type Actor%20Object%20Reference)))

(event EventTick
  (params (DeltaSeconds :type Float%20%28single-precision%29))
  (bind _boss_cube (Variables|Default|GetBoss%20Cube))
  (if (Variables|/Game/_Alex/Blueprints/AI/Enemies/BP_CubeEnemy.BP_CubeEnemy_C|GetIsDead _boss_cube)
    (Utilities|FlowControl|DoOnce false
      (:Completed
        (for _array_element (Variables|Default|GetDead%20Boss%20Spawn%20Object)
          (CallFunction|SetActorVisibility _array_element true)
          (bind _returnvalue (UserInterface|CreateWidget "/Game/_Alex/Blueprints/AI/Enemies/BossCube/WBP_DeadBossUI.WBP_DeadBossUI_C"))
          (bind _output_get (Variables|Default|SetDead%20Boss%20Widget _returnvalue))
          (UserInterface|Viewport|AddtoViewport _output_get 0)
          (Utilities|FlowControl|Delay 5.0)
          (Widget|RemovefromParent _output_get))))
    (else
      (switch Utilities|FlowControl|Switch|SwitchonEBossPhase (Variables|/Game/_Alex/Blueprints/AI/Enemies/BossCube/AIC_BossCube.AIC_BossCube_C|GetPhase (Variables|/Game/_Alex/Blueprints/AI/Enemies/BossCube/BP_BossCube.BP_BossCube_C|GetAIC%20Boss _boss_cube))
        (:NewEnumerator3
          (Utilities|FlowControl|DoOnce false
            (:Completed
              (Variables|/Game/_Alex/Blueprints/Trigger/Activator/BP_Gate.BP_Gate_C|SetOverride%20Activate (Variables|Default|GetFirst%20Gate) true))))
        (:NewEnumerator1
          (bind _completed (CallFunction|CheckEnemyWave))
          (if _completed
            (Default|EndShelter1 (Variables|Default|GetBoss%20Cube))))
        (:NewEnumerator5
          (bind _completed_2 (CallFunction|CheckEnemyWave))
          (if _completed_2
            (Default|EndShelter2 (Variables|Default|GetBoss%20Cube))))))))

(fn ConstructionScript)

(fn SpawnFirstWave
  (Variables|Default|SetEnemy%20Active true)
  (for _array_element (Variables|Default|GetEnemy%20Spawn%20Location)
    (bind _returnvalue (Game|SpawnActorfromClass (Variables|Default|GetEnemy) (Transformation|GetActorTransform _array_element) "Undefined" 0 0))
    (Pawn|SpawnDefaultController _returnvalue)
    (Utilities|Array|Add (Variables|Default|GetSpawned%20Enemies) _returnvalue)))

(fn CheckEnemyWave
  (bind _spawned_enemies (Variables|Default|GetSpawned%20Enemies))
  (Variables|Default|SetEnemy%20Controlled false)
  (if (Variables|Default|GetEnemy%20Active)
    (for _array_element _spawned_enemies
      (Utilities|IsValid (AI|GetAIController _array_element)
        (:Is%20Valid
          (return false))))
    (if (not (Variables|Default|GetEnemy%20Controlled))
      (Utilities|Array|Clear _spawned_enemies)
      (Variables|Default|SetEnemy%20Active false)
      (return true))
    (else
      (return false))))

(fn SpawnSecondWave
  (Variables|Default|SetEnemy%20Active true)
  (for _array_element (Variables|Default|GetEnemy%20Spawn%20Location%202)
    (bind _returnvalue (Game|SpawnActorfromClass (Variables|Default|GetEnemy) (Transformation|GetActorTransform _array_element) "Undefined" 0 0))
    (Pawn|SpawnDefaultController _returnvalue)
    (Utilities|Array|Add (Variables|Default|GetSpawned%20Enemies) _returnvalue))
  (for _array_element_2 (Variables|Default|GetEnemy%20Spawn%20Location%203)
    (bind _returnvalue_2 (Game|SpawnActorfromClass (Variables|Default|GetEnemy) (Transformation|GetActorTransform _array_element_2) "Undefined" 0 0))
    (Variables|/Game/_Alex/Blueprints/AI/Enemies/BP_CubeEnemy.BP_CubeEnemy_C|SetRange _returnvalue_2 true)
    (Pawn|SpawnDefaultController _returnvalue_2)
    (Utilities|Array|Add (Variables|Default|GetSpawned%20Enemies) _returnvalue_2)
    (AI|Components|Blackboard|SetValueasObject (AI|GetBlackboard _returnvalue_2) (Utilities|Name|MakeLiteralName "Player") (Variables|/Script/YDSU.MyGameInstanceCPP|GetCurrentCharacter (Variables|Default|GetGame%20Instance)))
    (for _array_element_3 (Variables|Default|GetPlatforms%20Phase%202)
      (Variables|/Game/_Alex/Blueprints/Trigger/Activator/BP_Gate.BP_Gate_C|SetOverride%20Activate _array_element_3 true)))
  (for _array_element_4 (Variables|Default|GetPlatforms%20Phase%202)
    (Variables|/Game/_Alex/Blueprints/Trigger/Activator/BP_Gate.BP_Gate_C|SetOverride%20Activate _array_element_4 true)))

(fn SetActorVisibility
  (params (Actor :type Actor%20Object%20Reference) (Visibility :type Boolean))
  (Rendering|SetActorHiddenInGame Actor (not Visibility))
  (Collision|SetActorEnableCollision Actor Visibility)
  (Actor|Tick|SetActorTickEnabled Actor Visibility))