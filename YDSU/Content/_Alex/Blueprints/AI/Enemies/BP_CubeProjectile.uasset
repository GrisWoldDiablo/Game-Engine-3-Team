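; Enemy cube projectile that damages MyCharacter on overlap and explodes.
; That overlap or any hit hides the cube, disables its collision, stops its movement and activates the explosion effect.
; The actor destroys itself when the trail particle system reports finished, not the explosion.
; Tick copies the actor's time dilation to both effects so they follow time changes applied to the projectile.
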(event Custom|Particle%20Finish
  (params (PSystem :type Particle%20System%20Component%20Object%20Reference))
  (Actor|DestroyActor))

(event Collision|EventActorBeginOverlap
  (params (OtherActor :type Actor%20Object%20Reference))
  (bind _cube (Variables|Default|GetCube))
  (bind _asmy_character (Utilities|Casting|CastToMyCharacter OtherActor))
  (Game|Damage|ApplyDamage _asmy_character (Math|Conversions|ToFloat(Integer) (Variables|Default|GetDamage)) 0 0)
  (EventDispatchers|AssignOnSystemFinished (Variables|Default|GetTrail) (delegate Custom|Particle%20Finish))
  (Rendering|SetVisibility _cube false false)
  (Collision|SetCollisionEnabled _cube "NoCollision")
  (Components|Movement|StopMovementImmediately (Variables|Default|GetProjectileMovement))
  (Components|Activation|Activate (Variables|Default|GetExplosion) false))

(event EventTick
  (params (DeltaSeconds :type Float%20%28single-precision%29))
  (bind _output_get (Variables|/Script/Engine.ParticleSystemComponent|SetCustomTimeDilation (Variables|Default|GetTrail) (Class|Actor|GetActorTimeDilation)))
  (Variables|/Script/Engine.ParticleSystemComponent|SetCustomTimeDilation (Variables|Default|GetExplosion) _output_get))

(event Collision|EventHit
  (params (MyComp :type Primitive%20Component%20Object%20Reference) (Other :type Actor%20Object%20Reference) (OtherComp :type Primitive%20Component%20Object%20Reference) (bSelfMoved :type Boolean) (HitLocation :type Vector :default "0, 0, 0") (HitNormal :type Vector :default "0, 0, 0") (NormalImpulse :type Vector :default "0, 0, 0") (Hit :type Hit%20Result%20Structure%20%28by%20ref%29))
  (bind _cube (Variables|Default|GetCube))
  (EventDispatchers|AssignOnSystemFinished (Variables|Default|GetTrail) (delegate Custom|Particle%20Finish))
  (Rendering|SetVisibility _cube false false)
  (Collision|SetCollisionEnabled _cube "NoCollision")
  (Components|Movement|StopMovementImmediately (Variables|Default|GetProjectileMovement))
  (Components|Activation|Activate (Variables|Default|GetExplosion) false))

(fn ConstructionScript)