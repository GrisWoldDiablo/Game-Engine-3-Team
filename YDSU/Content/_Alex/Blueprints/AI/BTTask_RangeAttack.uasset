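; Behavior tree task that makes BP_CubeEnemy perform a ranged throw attack on the player stored in the blackboard.
; If the player is visible, it plays AM_Throw and finishes at once, holding an Attacking flag until the montage completes.
; If the player is hidden, it clears the Player key and finishes successfully.
; Failed casts or an already active attack exit without finishing the task.
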(event EventReceiveExecuteAI
  (params (OwnerController :type AI%20Controller%20Object%20Reference) (ControlledPawn :type Pawn%20Object%20Reference))
  (bind _returnvalue (Utilities|Name|MakeLiteralName "Player"))
  (bind _asbp_cube_enemy (Utilities|Casting|CastToBP_CubeEnemy ControlledPawn))
  (if (not (Variables|Default|GetAttacking))
    (bind _asmy_character (Utilities|Casting|CastToMyCharacter (AI|Components|Blackboard|GetValueasObject (AI|GetBlackboard ControlledPawn) _returnvalue)))
    (if (not (Variables|/Script/Engine.Actor|GetbHidden _asmy_character))
      (Animation|Montage|PlayMontage (Variables|/Script/Engine.Character|GetMesh _asbp_cube_enemy) "/Game/_Alex/Animations/Enemies/Cube/Attack/AM_Throw.AM_Throw"
        (:then
          (Variables|Default|SetAttacking true))
        (:OnCompleted
          (Variables|Default|SetAttacking false)))
      (AI|BehaviorTree|FinishExecute true)
      (else
        (AI|Components|Blackboard|SetValueasObject (AI|GetBlackboard ControlledPawn) _returnvalue 0)
        (AI|BehaviorTree|FinishExecute true)))))