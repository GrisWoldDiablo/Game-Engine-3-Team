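; AI controller for enemy pawns that runs the BT_EnemyAI behavior tree and feeds its blackboard.
; On possess it starts the tree and, for a BP_CubeEnemy, stores the pawn's location as SpawnLocation.
; AI Perception updates set the Player key when a MyCharacter is successfully sensed.
; The controller never clears that key when sensing is lost.
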(event OnTargetPerceptionUpdated(AIPerception)
  (params (Actor :type Actor%20Object%20Reference) (Stimulus :type AI%20Stimulus%20Structure))
  (Utilities|Casting|CastToMyCharacter Actor)
  (if (.bsuccessfullysensed Stimulus)
    (AI|Components|Blackboard|SetValueasObject (Variables|Default|GetBlackboard) (Utilities|Name|MakeLiteralName "Player") Actor)))

(event EventBeginPlay)

(event EventTick
  (params (DeltaSeconds :type Float%20%28single-precision%29)))

(event EventPossess
  (params (PossessedPawn :type Pawn%20Object%20Reference))
  (AI|RunBehaviorTree "/Game/_Alex/Blueprints/AI/BT_EnemyAI.BT_EnemyAI")
  (bind _asbp_cube_enemy (Utilities|Casting|CastToBP_CubeEnemy PossessedPawn))
  (AI|Components|Blackboard|SetValueasVector (Variables|Default|GetBlackboard) (Utilities|Name|MakeLiteralName "SpawnLocation") (Transformation|GetActorLocation _asbp_cube_enemy)))

(fn ConstructionScript)