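; Player controller that lets the player swap between pyramid and ball characters, or join them into a third combined character when close together.
; Swapping possesses the other pawn, gives the old one a default controller, and uses timelines to interpolate the camera from the previous view.
; Join and split toggle visibility, collision and tick, teleport characters into place and copy camera boom settings.
; Tick draws a debug line when joining is possible.
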(event Custom|MoveSwapCamera
  (bind _interptarget (Variables|Default|GetInterpTarget))
  (bind _targettinterp (Variables|Default|GetTargetTinterp))
  (bind _returnvalue (Transformation|GetRelativeTransform _interptarget))
  (Transformation|SetRelativeTransform _interptarget (Class|KismetMathLibrary|TInterpto _returnvalue _targettinterp (Utilities|Time|GetWorldDeltaSeconds) (Variables|Default|GetInterpolationSpeed)) false false)
  (if (Class|KismetMathLibrary|NearlyEqualTransformTransform _returnvalue _targettinterp 0.1 0.01 0.01)
    (Transformation|SetRelativeTransform _interptarget _targettinterp false false)
    (Variables|Default|SetDoInterpCam false)))

(event EventBeginPlay
  ;[1 1 1] Begin Play
  ;[1 1 1] Populate MyCharacter Variables
  (bind _outactors (Actor|GetAllActorsOfClass "/Script/YDSU.MyCharacter"))
  (for _array_element _outactors
    (if (== (Utilities|GetClass _array_element) "/Game/_Alex/Blueprints/BP_ChaPy.BP_ChaPy_C")
      (Variables|Default|SetChaPy _array_element)
      (elif (== (Utilities|GetClass _array_element) "/Game/_Alex/Blueprints/BP_Character.BP_Character_C")
        (Variables|Default|SetChaBall _array_element)
        (else
          (Variables|Default|SetChaJoin _array_element))))))

(event EventTick
  (params (DeltaSeconds :type Float%20%28single-precision%29))
  ;[0.08142 1 0] Event Tick
  (if (Variables|Default|GetDoInterpCam)
    (CallFunction|MoveSwapCamera))
  ;[1 0.04395 0] Debug Line to Join
  (if (and (not (Variables|Default|GetJoin)) (<= (Transformation|GetDistanceTo (Variables|Default|GetChaPy) (Variables|Default|GetChaBall)) 2e+02))
    (Rendering|Debug|DrawDebugLine (Transformation|GetActorLocation (Variables|Default|GetChaPy)) (Transformation|GetActorLocation (Variables|Default|GetChaBall)) "(R=1.000000,G=0.000000,B=0.814425,A=1.000000)" 0.0 1e+01)))

(event Input|ActionEvents|InputActionSwap
  (params (Key :type Key%20Structure))
  (bind _chaball (Variables|Default|GetChaBall))
  (bind _chapy (Variables|Default|GetChaPy))
  (bind _transform (Variables|Default|GetTransform))
  (bind _topdowncameracomponent (Variables|/Script/YDSU.MyCharacter|GetTopDownCameraComponent _chapy))
  (bind _topdowncameracomponent_2 (Variables|/Script/YDSU.MyCharacter|GetTopDownCameraComponent _chaball))
  (bind _returnvalue (Transformation|GetRelativeTransform _topdowncameracomponent_2))
  (bind _returnvalue_2 (Class|KismetMathLibrary|NearlyEqualTransformTransform _returnvalue _transform 0.1 0.01 0.01))
  ;[1 1 1] Character Swap
  (:Pressed
    (if (not (Variables|Default|GetJoin))
      (if (== (Game|Player|GetPlayerPawn 0) (Variables|Default|GetChaPy))
        (Pawn|Possess _chaball)
        (Pawn|SpawnDefaultController _chapy)
        (Transformation|SetWorldTransform _topdowncameracomponent_2 (Transformation|GetWorldTransform _topdowncameracomponent) false false)
        (Timeline|To%20Ball%20TimeLine PlayFromStart
          (:Update
            (CallFunction|SwapCamPlayer (Variables|Default|GetChaBall))
            (if _returnvalue_2
              (Transformation|SetRelativeTransform _topdowncameracomponent_2 _transform false false)
              (Audio|Components|Audio|Stop (Variables|Default|GetTo%20Ball%20TimeLine))))
          (:Finished
            (if (not _returnvalue_2)
              (Components|Timeline|PlayfromStart (Variables|Default|GetTo%20Ball%20TimeLine)))))
        (else
          (Pawn|Possess _chapy)
          (Pawn|SpawnDefaultController _chaball)
          (Transformation|SetWorldTransform _topdowncameracomponent (Transformation|GetWorldTransform _topdowncameracomponent_2) false false)
          (Timeline|To%20Pyramid%20TimeLine PlayFromStart
            (:Update
              (CallFunction|SwapCamPlayer (Variables|Default|GetChaPy))
              (if (Class|KismetMathLibrary|NearlyEqualTransformTransform (Transformation|GetRelativeTransform _topdowncameracomponent) _transform 0.1 0.01 0.01)
                (Transformation|SetRelativeTransform _topdowncameracomponent _transform false false)
                (Audio|Components|Audio|Stop (Variables|Default|GetTo%20Pyramid%20TimeLine))))))))))

(event Input|ActionEvents|InputActionJoin
  (params (Key :type Key%20Structure))
  (bind _chaball (Variables|Default|GetChaBall))
  (bind _chapy (Variables|Default|GetChaPy))
  (bind _chajoin (Variables|Default|GetChaJoin))
  (bind _chajoin_2 (Variables|Default|GetChaJoin))
  (bind _chajoin_3 (Variables|Default|GetChaJoin))
  (bind _chaball_2 (Variables|Default|GetChaBall))
  (bind _returnvalue (Transformation|GetActorLocation _chajoin))
  ;[1 1 1] Join
  (:Pressed
    (if (not (Variables|Default|GetJoin))
      (if (<= (Transformation|GetDistanceTo (Variables|Default|GetChaPy) (Variables|Default|GetChaBall)) 2e+02)
        (CallFunction|HideActor _chajoin_3 false)
        (Pawn|Possess _chajoin_3)
        (CallFunction|HideActor _chaball_2 true)
        (CallFunction|HideActor (Variables|Default|GetChaPy) true)
        (Variables|Default|SetJoin true)
        (Transformation|SetActorLocation _chajoin_3 (Transformation|GetActorLocation _chaball_2) false true)
        (CallFunction|CopyCamValues _chaball_2 _chajoin_3))
      (else
        ;[1 1 1] Split
        (Pawn|Possess _chaball)
        (Pawn|SpawnDefaultController _chapy)
        (CallFunction|HideActor _chajoin_2 true)
        (Transformation|SetActorLocation _chaball _returnvalue false true)
        (Transformation|SetActorLocation _chapy _returnvalue false true)
        (CallFunction|HideActor _chaball false)
        (CallFunction|HideActor _chapy false)
        (CallFunction|CopyCamValues _chajoin_2 _chaball)
        (CallFunction|CopyCamValues _chajoin_2 _chapy)
        (Variables|Default|SetJoin false)))))

(fn ConstructionScript)

(fn HideActor
  (params (Actor :type Actor%20Object%20Reference) (ToHide :type Boolean))
  (bind _returnvalue (not ToHide))
  (Rendering|SetActorHiddenInGame Actor ToHide)
  (Collision|SetActorEnableCollision Actor _returnvalue)
  (Actor|Tick|SetActorTickEnabled Actor _returnvalue))

(fn CopyCamValues
  (params (From%20Char :type My%20Character%20Object%20Reference%20%28by%20ref%29) (To%20Char :type My%20Character%20Object%20Reference%20%28by%20ref%29))
  (bind _cameraboom (Variables|/Script/YDSU.MyCharacter|GetCameraBoom To%20Char))
  (bind _output_get (Variables|/Script/YDSU.MyCharacter|SetCameraRotator To%20Char (Variables|/Script/YDSU.MyCharacter|GetCameraRotator From%20Char)))
  (bind _output_get_2 (Variables|/Script/YDSU.MyCharacter|SetCameraLenght To%20Char (Variables|/Script/YDSU.MyCharacter|GetCameraLenght From%20Char)))
  (bind _output_get_3 (Variables|/Script/YDSU.MyCharacter|SetCamLagDistance To%20Char (Variables|/Script/YDSU.MyCharacter|GetCamLagDistance From%20Char)))
  (bind _output_get_4 (Variables|/Script/YDSU.MyCharacter|SetCamLagSpeed To%20Char (Variables|/Script/YDSU.MyCharacter|GetCamLagDistance From%20Char)))
  (Transformation|SetRelativeRotation _cameraboom _output_get false false)
  (Variables|/Script/Engine.SpringArmComponent|SetTargetArmLength _cameraboom _output_get_2)
  (Variables|/Script/Engine.SpringArmComponent|SetCameraLagMaxDistance _cameraboom _output_get_3)
  (Variables|/Script/Engine.SpringArmComponent|SetCameraLagSpeed _cameraboom _output_get_4))

(fn SwapCamPlayer
  (params (To%20Char :type My%20Character%20Object%20Reference%20%28by%20ref%29))
  (bind _topdowncameracomponent (Variables|/Script/YDSU.MyCharacter|GetTopDownCameraComponent To%20Char))
  (Transformation|SetRelativeTransform _topdowncameracomponent (Class|KismetMathLibrary|TInterpto (Transformation|GetRelativeTransform _topdowncameracomponent) (Math|Transform|MakeTransform "0, 0, 0") (Utilities|Time|GetWorldDeltaSeconds) (Variables|Default|GetInterpolationSpeed)) false false))