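; Player controller that manages switching between the Ball, Pyramid and Join characters, as each level's available-character setting allows.
; BeginPlay takes the characters from MyGameInstance, then sets visibility and possession; Swap blends the camera and hands the released character a default controller.
; Join merges the nearby pair or splits them by toggling visibility, collision and tick and copying camera values.
; Slow triggers a test Pyramid finisher with time dilation and an enemy camera.
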(event EventBeginPlay
  ;[1 1 1] Begin Play
  (Development|PrintString (Utilities|String|EnumtoString (Variables|Default|GetAvailable%20Characters)))
  ;[1 1 1] Populate MyCharacter Variables
  (bind _asmy_game_instance (Utilities|Casting|CastToMyGameInstance (Game|GetGameInstance)))
  (bind _output_get (Variables|Default|SetMyGameInstance _asmy_game_instance))
  (Variables|Default|SetChaPy (Variables|/Game/_Alex/Blueprints/MyGameInstance.MyGameInstance_C|GetCharacter%20Pyramid _output_get))
  (Variables|Default|SetChaJoin (Variables|/Game/_Alex/Blueprints/MyGameInstance.MyGameInstance_C|GetCharacter%20Join _output_get))
  (Variables|Default|SetChaBall (Variables|/Game/_Alex/Blueprints/MyGameInstance.MyGameInstance_C|GetCharacter%20Ball _output_get))
  ;[1 1 1] Initialize Characters per Level specification
  (CallFunction|InitCharacters))

(event EventTick
  (params (DeltaSeconds :type Float%20%28single-precision%29))
  ;[0.08142 1 0] Event Tick
  ;[1 0.04395 0] Debug Line to Join
  (if (Math|Boolean|ANDBoolean (not (Variables|Default|GetIs%20Join)) (<= (Transformation|GetDistanceTo (Variables|Default|GetChaPy) (Variables|Default|GetChaBall)) 2e+02) (Utilities|Enum|Equal(Enum) (Variables|Default|GetAvailable%20Characters) "NewEnumerator4"))
    (Rendering|Debug|DrawDebugLine (Transformation|GetActorLocation (Variables|Default|GetChaPy)) (Transformation|GetActorLocation (Variables|Default|GetChaBall)) "(R=1.000000,G=0.000000,B=0.814425,A=1.000000)" 0.0 1e+01)))

(event Input|ActionEvents|InputActionSwap
  (params (Key :type Key%20Structure))
  (bind _chaball (Variables|Default|GetChaBall))
  (bind _chapy (Variables|Default|GetChaPy))
  (bind _available_characters (Variables|Default|GetAvailable%20Characters))
  ;[1 1 1] Character Swap
  (:Pressed
    (if (and (not (Variables|Default|GetIs%20Join)) (or (Utilities|Enum|Equal(Enum) _available_characters "NewEnumerator3") (Utilities|Enum|Equal(Enum) _available_characters "NewEnumerator4")))
      (if (== (Variables|Default|GetCurrent%20Character) (Variables|Default|GetChaPy))
        (Game|Player|SetViewTargetwithBlend _chaball (Variables|Default|GetCamBlenTime) "VTBlend_Cubic" 0.0 true)
        (Pawn|Possess _chaball)
        (Pawn|SpawnDefaultController _chapy)
        (Variables|Default|SetCurrent%20Character _chaball)
        (else
          (Game|Player|SetViewTargetwithBlend _chapy (Variables|Default|GetCamBlenTime) "VTBlend_Cubic" 0.0 true)
          (Pawn|Possess _chapy)
          (Pawn|SpawnDefaultController _chaball)
          (Variables|Default|SetCurrent%20Character _chapy))))))

(event Input|ActionEvents|InputActionSlow
  (params (Key :type Key%20Structure))
  ;[1 1 1] Finisher Camera Testing
  (:Pressed
    (bind _asbp_pyramid (Utilities|Casting|CastToBP_Pyramid (Game|Player|GetPlayerPawn 0)))
    (if (Variables|/Game/_Alex/Blueprints/Character/BP_Pyramid.BP_Pyramid_C|GetOverLapEnemy _asbp_pyramid)
      (Character|Jump _asbp_pyramid)
      (Utilities|FlowControl|Delay 0.2)
      (Pawn|Components|CharacterMovement|SetMovementMode (Variables|/Script/Engine.Character|GetCharacterMovement _asbp_pyramid) "MOVE_None" 0)
      (Utilities|Time|SetGlobalTimeDilation 0.2)
      (Game|Player|SetViewTargetwithBlend (Variables|/Game/_Alex/Blueprints/Character/BP_Pyramid.BP_Pyramid_C|GetEnemy _asbp_pyramid) 1.0 "VTBlend_Cubic" 2.0 true)
      (Utilities|FlowControl|Delay 1.0)
      (Default|FInisherCam (Variables|/Game/_Alex/Blueprints/Character/BP_Pyramid.BP_Pyramid_C|GetEnemy _asbp_pyramid))
      (Utilities|FlowControl|Delay 1.0)
      (Utilities|Time|SetGlobalTimeDilation 1.0)
      (Pawn|Components|CharacterMovement|SetMovementMode (Variables|/Script/Engine.Character|GetCharacterMovement _asbp_pyramid) "MOVE_Walking" 0)
      (Game|Player|SetViewTargetwithBlend _asbp_pyramid 1.0 "VTBlend_Linear" 2.0 true)
      (Utilities|FlowControl|Delay 1.0)
      (Actor|DestroyActor (Variables|/Game/_Alex/Blueprints/Character/BP_Pyramid.BP_Pyramid_C|GetEnemy _asbp_pyramid)))))

(event Input|ActionEvents|InputActionJoin
  (params (Key :type Key%20Structure))
  (bind _chaball (Variables|Default|GetChaBall))
  (bind _chapy (Variables|Default|GetChaPy))
  (bind _chajoin (Variables|Default|GetChaJoin))
  (bind _chajoin_2 (Variables|Default|GetChaJoin))
  (bind _chaball_2 (Variables|Default|GetChaBall))
  (bind _returnvalue (Transformation|GetActorLocation _chajoin))
  ;[1 1 1] Join
  (:Pressed
    (if (and (not (Variables|Default|GetIs%20Join)) (Utilities|Enum|Equal(Enum) (Variables|Default|GetAvailable%20Characters) "NewEnumerator4"))
      (if (<= (Transformation|GetDistanceTo (Variables|Default|GetChaPy) (Variables|Default|GetChaBall)) 2e+02)
        (Pawn|Possess _chajoin_2)
        (CallFunction|SetActorVisibility _chajoin_2 true)
        (CallFunction|SetActorVisibility _chaball_2 false)
        (CallFunction|SetActorVisibility (Variables|Default|GetChaPy) false)
        (Variables|Default|SetIs%20Join true)
        (Transformation|SetActorLocation _chajoin_2 (Transformation|GetActorLocation _chaball_2) false false)
        (CallFunction|CopyCamValues _chaball_2 _chajoin_2 false)
        (Game|Player|SetViewTargetwithBlend _chajoin_2 (Variables|Default|GetCamBlenTime) "VTBlend_Cubic" 0.0 true))
      (else
        ;[1 1 1] Split
        (if (Utilities|Enum|Equal(Enum) (Variables|Default|GetAvailable%20Characters) "NewEnumerator4")
          (Pawn|Possess _chapy)
          (Variables|Default|SetCurrent%20Character _chapy)
          (CallFunction|SetActorVisibility _chapy true)
          (CallFunction|SetActorVisibility _chaball true)
          (CallFunction|SetActorVisibility _chajoin false)
          (Transformation|SetActorLocation _chaball _returnvalue false true)
          (Transformation|SetActorLocation _chapy _returnvalue false true)
          (CallFunction|CopyCamValues _chajoin _chaball true)
          (CallFunction|CopyCamValues _chajoin _chapy true)
          (Variables|Default|SetIs%20Join false)
          (Game|Player|SetViewTargetwithBlend _chapy (Variables|Default|GetCamBlenTime) "VTBlend_Cubic" 0.0 true))))))

(fn ConstructionScript)

(fn SetActorVisibility
  (params (Actor :type Actor%20Object%20Reference%20%28by%20ref%29) (Visibility :type Boolean))
  (Rendering|SetActorHiddenInGame Actor (not Visibility))
  (Collision|SetActorEnableCollision Actor Visibility)
  (Actor|Tick|SetActorTickEnabled Actor Visibility))

(fn CopyCamValues
  (params (From%20Char :type My%20Character%20Object%20Reference%20%28by%20ref%29) (To%20Char :type My%20Character%20Object%20Reference%20%28by%20ref%29) (ChangeNow :type Boolean))
  (bind _cameraboom (Variables|/Script/YDSU.MyCharacter|GetCameraBoom To%20Char))
  (bind _output_get (Variables|/Script/YDSU.MyCharacter|SetCameraRotator To%20Char (Variables|/Script/YDSU.MyCharacter|GetCameraRotator From%20Char)))
  (bind _output_get_2 (Variables|/Script/YDSU.MyCharacter|SetCameraLenght To%20Char (Variables|/Script/YDSU.MyCharacter|GetCameraLenght From%20Char)))
  (bind _output_get_3 (Variables|/Script/YDSU.MyCharacter|SetCamLagDistance To%20Char (Variables|/Script/YDSU.MyCharacter|GetCamLagDistance From%20Char)))
  (bind _output_get_4 (Variables|/Script/YDSU.MyCharacter|SetCamLagSpeed To%20Char (Variables|/Script/YDSU.MyCharacter|GetCamLagDistance From%20Char)))
  (Transformation|SetRelativeRotation _cameraboom _output_get false false)
  (Variables|/Script/Engine.SpringArmComponent|SetTargetArmLength _cameraboom _output_get_2)
  (Variables|/Script/Engine.SpringArmComponent|SetCameraLagMaxDistance _cameraboom _output_get_3)
  (Variables|/Script/Engine.SpringArmComponent|SetCameraLagSpeed _cameraboom _output_get_4))

(fn ChangeCamera
  (params (ObjectToMove :type Scene%20Component%20Object%20Reference) (TargetLocation :type Transform) (StartLocation :type Scene%20Component%20Object%20Reference))
  (Variables|Default|SetInterpTarget ObjectToMove)
  (Variables|Default|SetTargetTinterp TargetLocation)
  (Variables|Default|SetOriginCam (Transformation|GetWorldTransform StartLocation))
  (Variables|Default|SetDoInterpCam true)
  (Variables|Default|SetIsInterpolating false))

(fn DotheCameraInterpolation
  (bind _interptarget (Variables|Default|GetInterpTarget))
  (bind _targettinterp (Variables|Default|GetTargetTinterp))
  (bind _returnvalue (Transformation|GetRelativeTransform _interptarget))
  (if (Variables|Default|GetIsInterpolating)
    _
    (else
      (Transformation|SetWorldTransform (Variables|Default|GetInterpTarget) (Variables|Default|GetOriginCam) false true)
      (Variables|Default|SetIsInterpolating true)))
  (Transformation|SetRelativeTransform _interptarget (Class|KismetMathLibrary|TInterpto _returnvalue _targettinterp (Utilities|Time|GetWorldDeltaSeconds) (Variables|Default|GetInterpolationSpeed)) false false)
  (if (Class|KismetMathLibrary|NearlyEqualTransformTransform _returnvalue _targettinterp 0.1 0.01 0.01)
    (Transformation|SetRelativeTransform _interptarget _targettinterp false false)
    (Variables|Default|SetDoInterpCam false)
    (Variables|Default|SetIsInterpolating false)
    (return true)
    (else
      (return false))))

(fn InitCharacters
  (switch Utilities|FlowControl|Switch|SwitchonCharacterType (Variables|Default|GetAvailable%20Characters)
    (:NewEnumerator0
      (CallFunction|SetActorVisibility (Variables|Default|GetChaBall) true)
      (CallFunction|SetActorVisibility (Variables|Default|GetChaPy) false)
      (CallFunction|SetActorVisibility (Variables|Default|GetChaJoin) false)
      (Pawn|Possess (Variables|Default|GetChaBall) :!label _label))
    (:NewEnumerator1
      (CallFunction|SetActorVisibility (Variables|Default|GetChaBall) false)
      (CallFunction|SetActorVisibility (Variables|Default|GetChaPy) true)
      (CallFunction|SetActorVisibility (Variables|Default|GetChaJoin) false)
      (Pawn|Possess (Variables|Default|GetChaPy)))
    (:NewEnumerator2
      (Variables|Default|SetIs%20Join true :!label _label_2)
      (CallFunction|SetActorVisibility (Variables|Default|GetChaBall) false)
      (CallFunction|SetActorVisibility (Variables|Default|GetChaPy) false)
      (CallFunction|SetActorVisibility (Variables|Default|GetChaJoin) true)
      (Pawn|Possess (Variables|Default|GetChaJoin)))
    (:NewEnumerator3
      (CallFunction|SetActorVisibility (Variables|Default|GetChaBall) true)
      (CallFunction|SetActorVisibility (Variables|Default|GetChaPy) true)
      (CallFunction|SetActorVisibility (Variables|Default|GetChaJoin) false)
      (goto _label))
    (:NewEnumerator4
      (goto _label_2)))
  (bind _asmy_character (Utilities|Casting|CastToMyCharacter (Pawn|GetControlledPawn (Game|GetPlayerController 0))))
  (bind _output_get (Variables|Default|SetCurrent%20Character _asmy_character))
  (Game|Player|SetViewTargetwithBlend _output_get 0.0 "VTBlend_Linear" 0.0 false))