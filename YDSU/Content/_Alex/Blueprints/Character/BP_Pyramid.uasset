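; BP_Pyramid is a damageable pyramid Blueprint that tracks its own hit points.
; On BeginPlay it caches the cast MyGameInstance and sets HP from StartHP, stopping if the cast fails.
; AnyDamage prints a debug string and subtracts truncated damage from HP, with no death handling.
; A disconnected node that would write PyramidHP to the game instance's CurrentChar never runs.
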(event EventBeginPlay
  (bind _asmy_game_instance (Utilities|Casting|CastToMyGameInstance (Game|GetGameInstance)))
  (Variables|Default|SetMyGameInstance _asmy_game_instance)
  (Variables|Default|SetHP (Variables|Default|GetStartHP)))

(event EventTick
  (params (DeltaSeconds :type Float%20%28single-precision%29)))

(event Game|Damage|EventAnyDamage
  (params (Damage :type Float%20%28single-precision%29) (DamageType :type Damage%20Type%20Object%20Reference) (InstigatedBy :type Controller%20Object%20Reference) (DamageCauser :type Actor%20Object%20Reference))
  (Development|PrintString "HURT PYRAMID")
  (Variables|Default|SetHP (- (Variables|Default|GetHP) (Math|Float|Truncate Damage))))

(event Input|ActionEvents|InputActionHurt
  (params (Key :type Key%20Structure)))

(fn ConstructionScript)