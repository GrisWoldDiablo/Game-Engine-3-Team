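; Ball character that toggles between walking movement and a simulated physics mode, and tracks HP that incoming damage reduces.
; The toggle swaps CharacterMovement for capsule physics and back, while a timeline blends a dynamic material's Lerp parameter to show the mode.
; Outside physics mode, movement axis events fake rolling by rotating the mesh around an axis derived from planar velocity, easing back when stopped.
; BeginPlay also caches the game instance and adds a debug UI.
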(event Custom|TurnPhysic
  (bind _charactermovement (Variables|Character|GetCharacterMovement))
  (bind _capsulecomponent (Variables|Default|GetCapsuleComponent))
  ;[1 1 1] Set Physic mode
  (if (Variables|Default|GetPhysicOn)
    (Pawn|Components|CharacterMovement|SetMovementMode _charactermovement "MOVE_Walking" 0)
    (Physics|SetSimulatePhysics _capsulecomponent false)
    (Variables|Default|SetPhysicOn false)
    (Transformation|SetWorldRotation (Variables|Default|GetCapsuleComponent) "0, 0, 0" false false)
    (CallFunction|InterpMatReverse)
    (else
      (Pawn|Components|CharacterMovement|DisableMovement _charactermovement)
      (Physics|SetSimulatePhysics _capsulecomponent true)
      (Variables|Default|SetPhysicOn true)
      (CallFunction|InterpMat))))

(event Custom|Interp%20Mat
  ;[1 1 1] Interpolate material
  (bind _value (Timeline|Mat%20Interp%20Timeline PlayFromStart)
    (:Update
      (Rendering|Material|SetScalarParameterValue (Variables|Default|GetMaterial) "Lerp" _value :!class /Script/Engine.MaterialInstanceDynamic))))

(event Custom|Interp%20Mat%20Reverse
  ;[1 1 1] Interpolate material
  (bind _value (Timeline|Mat%20Interp%20Timeline Reverse)
    (:Update
      (Rendering|Material|SetScalarParameterValue (Variables|Default|GetMaterial) "Lerp" _value :!class /Script/Engine.MaterialInstanceDynamic))))

(event Game|Damage|EventAnyDamage
  (params (Damage :type Float%20%28single-precision%29) (DamageType :type Damage%20Type%20Object%20Reference) (InstigatedBy :type Controller%20Object%20Reference) (DamageCauser :type Actor%20Object%20Reference))
  (Development|PrintString "HURT BALL")
  (Variables|Default|SetHP (- (Variables|Default|GetHP) (Math|Float|Truncate Damage))))

(event EventBeginPlay
  ;[1 1 1] On Begin Play
  (bind _asmy_game_instance (Utilities|Casting|CastToMyGameInstance (Game|GetGameInstance)))
  (Variables|Default|SetMyGameInstance _asmy_game_instance)
  (bind _output_get (Variables|Default|SetMaxHP (Variables|Default|GetStartHP)))
  (Variables|Default|SetHP _output_get)
  (bind _returnvalue (UserInterface|CreateWidget "/Game/_Alex/Blueprints/UI/WBP_DebugUI.WBP_DebugUI_C"))
  (bind _output_get_2 (Variables|Default|SetUIDebug _returnvalue))
  (UserInterface|Viewport|AddtoPlayerScreen _output_get_2)
  (bind _returnvalue_2 (Rendering|Material|CreateDynamicMaterialInstance (Variables|Character|GetMesh) 0 0 "None" :!class /Script/Engine.PrimitiveComponent))
  (Variables|Default|SetMaterial _returnvalue_2))

(event Input|ActionEvents|InputActionTurnPhysic
  (params (Key :type Key%20Structure))
  (bind _charactermovement (Variables|Character|GetCharacterMovement))
  (bind _capsulecomponent (Variables|Default|GetCapsuleComponent))
  ;[1 1 1] Set Physic mode
  (:Pressed
    (if (Variables|Default|GetPhysicOn)
      (Pawn|Components|CharacterMovement|SetMovementMode _charactermovement "MOVE_Walking" 0)
      (Physics|SetSimulatePhysics _capsulecomponent false)
      (Variables|Default|SetPhysicOn false)
      (Transformation|SetWorldRotation (Variables|Default|GetCapsuleComponent) "0, 0, 0" false false)
      (CallFunction|InterpMatReverse)
      (else
        (Pawn|Components|CharacterMovement|DisableMovement _charactermovement)
        (Physics|SetSimulatePhysics _capsulecomponent true)
        (Variables|Default|SetPhysicOn true)
        (CallFunction|InterpMat)))))

(event Input|ActionEvents|InputActionHurt
  (params (Key :type Key%20Structure)))

(event Input|AxisEvents|InputAxisMoveForward
  (params (AxisValue :type Float%20%28single-precision%29))
  (bind _returnvalue (Transformation|GetVelocity))
  (bind _mesh (Variables|Character|GetMesh))
  ;[1 1 1] Rotate Mesh Following the velocity
  (if (not (Variables|Default|GetPhysicOn))
    (bind _output_get (Variables|Default|SetPlanar%20Velocity (Math|Vector|MakeVector (.x _returnvalue) (.y _returnvalue) 0.0)))
    (bind _output_get_2 (Variables|Default|SetHorizontal%20Speed (Math|Vector|VectorLength _output_get)))
    (Math|Float|CompareFloat _output_get_2 0.0
      (:>
        (bind _output_get_3 (Variables|Default|SetHorizontal%20Rotation%20Amount (|(RotationAmount+((PI/Ratio)*DeltaSecond)) (Math|Trig|GetPI) (Variables|Default|GetHorizontal%20Rotation%20Amount) (Variables|Default|GetHorizontal%20Rotation%20Ratio) (Utilities|Time|GetWorldDeltaSeconds))))
        (Transformation|SetWorldRotation (Variables|Character|GetMesh) (Math|Vector|RotatorfromAxisandAngle (Math|Vector|GetRightVector (Math|Rotator|MakeRotfromX (Math|Vector|Normalize (Variables|Default|GetPlanar%20Velocity)))) _output_get_3) false false))
      (:==
        (Transformation|SetWorldRotation _mesh (Math|Interpolation|RInterpTo (Transformation|GetWorldRotation _mesh) "0, 0, 0" (Utilities|Time|GetWorldDeltaSeconds) 5.0) false true)
        (Variables|Default|SetHorizontal%20Rotation%20Amount 0.0)))))

(event Input|AxisEvents|InputAxisMoveRight
  (params (AxisValue :type Float%20%28single-precision%29))
  (bind _returnvalue (Transformation|GetVelocity))
  (bind _mesh (Variables|Character|GetMesh))
  ;[1 1 1] Rotate Mesh Following the velocity
  (if (not (Variables|Default|GetPhysicOn))
    (bind _output_get (Variables|Default|SetPlanar%20Velocity (Math|Vector|MakeVector (.x _returnvalue) (.y _returnvalue) 0.0)))
    (bind _output_get_2 (Variables|Default|SetHorizontal%20Speed (Math|Vector|VectorLength _output_get)))
    (Math|Float|CompareFloat _output_get_2 0.0
      (:>
        (bind _output_get_3 (Variables|Default|SetHorizontal%20Rotation%20Amount (|(RotationAmount+((PI/Ratio)*DeltaSecond)) (Math|Trig|GetPI) (Variables|Default|GetHorizontal%20Rotation%20Amount) (Variables|Default|GetHorizontal%20Rotation%20Ratio) (Utilities|Time|GetWorldDeltaSeconds))))
        (Transformation|SetWorldRotation (Variables|Character|GetMesh) (Math|Vector|RotatorfromAxisandAngle (Math|Vector|GetRightVector (Math|Rotator|MakeRotfromX (Math|Vector|Normalize (Variables|Default|GetPlanar%20Velocity)))) _output_get_3) false false))
      (:==
        (Transformation|SetWorldRotation _mesh (Math|Interpolation|RInterpTo (Transformation|GetWorldRotation _mesh) "0, 0, 0" (Utilities|Time|GetWorldDeltaSeconds) 5.0) false true)
        (Variables|Default|SetHorizontal%20Rotation%20Amount 0.0)))))

(fn ConstructionScript)