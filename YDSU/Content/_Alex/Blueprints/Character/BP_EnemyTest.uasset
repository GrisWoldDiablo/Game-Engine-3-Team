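; BP_EnemyTest is a test enemy character with camera-relative movement input and a cinematic camera move for finishers.
; MoveForward and MoveRight axes drive movement along the Camera's yaw, ignoring pitch and roll.
; FInisherCam plays a timeline that slides the CC component along the Spline by percentage of its length, turning it toward the actor root each update.
; The construction script places CC at the first spline point, facing the root.
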(event Custom|FInisherCam
  (bind _cc (Variables|Default|GetCC))
  (bind _spline (Variables|Default|GetSpline))
  (bind _track_percentage (Timeline|Timeline_0 PlayFromStart)
    (:Update
      (Transformation|SetWorldTransform _cc (Spline|GetTransformatDistanceAlongSpline _spline (* _track_percentage (Spline|GetSplineLength _spline)) "World" false) false false)
      (Transformation|SetWorldRotation _cc (Math|Rotator|FindLookatRotation (Transformation|GetWorldLocation _cc) (Transformation|GetWorldLocation (Variables|Transformation|GetRootComponent))) false false))))

(event EventBeginPlay)

(event Collision|EventActorBeginOverlap
  (params (OtherActor :type Actor%20Object%20Reference)))

(event EventTick
  (params (DeltaSeconds :type Float%20%28single-precision%29)))

(event Input|AxisEvents|InputAxisMoveForward
  (params (AxisValue :type Float%20%28single-precision%29))
  (Pawn|Input|AddMovementInput (Math|Vector|GetForwardVector (Math|Rotator|MakeRotator 0.0 0.0 (.Yaw (Math|Rotator|BreakRotator (Transformation|GetWorldRotation (Variables|Default|GetCamera)))))) AxisValue false))

(event Input|AxisEvents|InputAxisMoveRight
  (params (AxisValue :type Float%20%28single-precision%29))
  (Pawn|Input|AddMovementInput (Math|Vector|GetRightVector (Math|Rotator|MakeRotator 0.0 0.0 (.Yaw (Math|Rotator|BreakRotator (Transformation|GetWorldRotation (Variables|Default|GetCamera)))))) AxisValue false))

(fn ConstructionScript
  (bind _cc (Variables|Default|GetCC))
  (Transformation|SetWorldTransform _cc (Math|Transform|MakeTransform (.location (Spline|GetTransformatSplinePoint (Variables|Default|GetSpline) 0 "World" false)) (Transformation|GetWorldRotation _cc) "1,1,1") false false)
  (Transformation|SetWorldRotation _cc (Math|Rotator|FindLookatRotation (Transformation|GetWorldLocation _cc) (Transformation|GetWorldLocation (Variables|Transformation|GetRootComponent))) false false))