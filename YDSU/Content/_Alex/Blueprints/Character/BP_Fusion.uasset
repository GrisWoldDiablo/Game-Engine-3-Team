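; Player character Blueprint for melee combat with cyclable attack montages, enemy targeting and a charge montage played on the Slow input.
; TargetZone overlaps maintain the in-range BP_CubeEnemy list in MyGameInstance, which also stores the current target.
; Targeting toggles onto the nearest listed enemy; attacking auto-targets, and Tick retargets when the target becomes invalid.
; Capsule overlaps apply damage directly to the overlapped actor, independent of attack state.
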(event OnComponentBeginOverlap(TargetZone)
  (params (OverlappedComponent :type Primitive%20Component%20Object%20Reference) (OtherActor :type Actor%20Object%20Reference) (OtherComp :type Primitive%20Component%20Object%20Reference) (OtherBodyIndex :type Integer) (bFromSweep :type Boolean) (SweepResult :type Hit%20Result%20Structure%20%28by%20ref%29))
  ;[1 1 1] Add enemy to the list who entered range.
  (bind _asbp_cube_enemy (Utilities|Casting|CastToBP_CubeEnemy OtherActor))
  (Utilities|Array|Add (Variables|/Game/_Alex/Blueprints/Utility/MyGameInstance.MyGameInstance_C|GetEnemies%20In%20Range (Variables|Default|GetMyGameInstance)) _asbp_cube_enemy)
  (Development|PrintString (Utilities|GetDisplayName _asbp_cube_enemy)))

(event OnComponentEndOverlap(TargetZone)
  (params (OverlappedComponent :type Primitive%20Component%20Object%20Reference) (OtherActor :type Actor%20Object%20Reference) (OtherComp :type Primitive%20Component%20Object%20Reference) (OtherBodyIndex :type Integer))
  ;[1 1 1] Remove enemy that can be targeted from the list since it left range.
  (bind _asbp_cube_enemy (Utilities|Casting|CastToBP_CubeEnemy OtherActor))
  (Utilities|Array|RemoveItem (Variables|/Game/_Alex/Blueprints/Utility/MyGameInstance.MyGameInstance_C|GetEnemies%20In%20Range (Variables|Default|GetMyGameInstance)) _asbp_cube_enemy))

(event OnComponentBeginOverlap(Capsule)
  (params (OverlappedComponent :type Primitive%20Component%20Object%20Reference) (OtherActor :type Actor%20Object%20Reference) (OtherComp :type Primitive%20Component%20Object%20Reference) (OtherBodyIndex :type Integer) (bFromSweep :type Boolean) (SweepResult :type Hit%20Result%20Structure%20%28by%20ref%29))
  ;[1 1 1] Damage enemy
  (Game|Damage|ApplyDamage OtherActor 0.25 0 0))

(event Custom|Target%20Enemy
  (bind _self self)
  (bind _mygameinstance (Variables|Default|GetMyGameInstance))
  (bind _enemies_in_range (Variables|/Game/_Alex/Blueprints/Utility/MyGameInstance.MyGameInstance_C|GetEnemies%20In%20Range _mygameinstance))
  ;[1 1 1] Target Enemy
  (bind _output_get (Variables|/Game/_Alex/Blueprints/Utility/MyGameInstance.MyGameInstance_C|SetEnemy%20Targeted _mygameinstance (Utilities|Array|Get(acopy) _enemies_in_range)))
  (for _array_element _enemies_in_range
    (Math|Float|CompareFloat (Transformation|GetDistanceTo _array_element _self) (Transformation|GetDistanceTo _output_get _self)
      (:==
        _)
      (:<
        _))
    (Variables|/Game/_Alex/Blueprints/Utility/MyGameInstance.MyGameInstance_C|SetEnemy%20Targeted (Variables|Default|GetMyGameInstance) _array_element)
    (Variables|Default|SetIsTargeting true)))

(event EventBeginPlay
  (bind _asmy_game_instance (Utilities|Casting|CastToMyGameInstance (Game|GetGameInstance)))
  (Variables|Default|SetMyGameInstance _asmy_game_instance))

(event EventTick
  (params (DeltaSeconds :type Float%20%28single-precision%29))
  (bind _self self)
  (bind _mygameinstance (Variables|Default|GetMyGameInstance))
  (bind _enemies_in_range (Variables|/Game/_Alex/Blueprints/Utility/MyGameInstance.MyGameInstance_C|GetEnemies%20In%20Range _mygameinstance))
  ;[1 1 1] Retarget
  (if (and (Variables|Default|GetIsTargeting) (not (Utilities|IsValid (Variables|/Game/_Alex/Blueprints/Utility/MyGameInstance.MyGameInstance_C|GetEnemy%20Targeted (Variables|Default|GetMyGameInstance)))))
    ;[1 1 1] Target Enemy
    (bind _output_get (Variables|/Game/_Alex/Blueprints/Utility/MyGameInstance.MyGameInstance_C|SetEnemy%20Targeted _mygameinstance (Utilities|Array|Get(acopy) _enemies_in_range)))
    (for _array_element _enemies_in_range
      (Math|Float|CompareFloat (Transformation|GetDistanceTo _array_element _self) (Transformation|GetDistanceTo _output_get _self)
        (:==
          _)
        (:<
          _))
      (Variables|/Game/_Alex/Blueprints/Utility/MyGameInstance.MyGameInstance_C|SetEnemy%20Targeted (Variables|Default|GetMyGameInstance) _array_element)
      (Variables|Default|SetIsTargeting true))))

(event Input|ActionEvents|InputActionAttack
  (params (Key :type Key%20Structure))
  ;[1 1 1] Attack Stabbing
  (:Pressed
    (if (not (Variables|Default|GetAttacking))
      (if (Variables|Default|GetIsTargeting)
        _
        (else
          (CallFunction|TargetEnemy)))
      (Variables|Default|SetAttacking true)
      (Animation|Montage|PlayMontage (Variables|Character|GetMesh) (Utilities|Array|Get(acopy) (Variables|Default|GetAttacks) (Variables|Default|GetAttackIndex))
        (:OnCompleted
          (Variables|Default|SetAttacking false))))))

(event Input|ActionEvents|InputActionTarget
  (params (Key :type Key%20Structure))
  (bind _self self)
  (bind _mygameinstance (Variables|Default|GetMyGameInstance))
  (bind _enemies_in_range (Variables|/Game/_Alex/Blueprints/Utility/MyGameInstance.MyGameInstance_C|GetEnemies%20In%20Range _mygameinstance))
  ;[1 1 1] Target Enemy
  (:Pressed
    (Utilities|IsValid (Variables|/Game/_Alex/Blueprints/Utility/MyGameInstance.MyGameInstance_C|GetEnemy%20Targeted _mygameinstance)
      (:Is%20Valid
        (Variables|/Game/_Alex/Blueprints/Utility/MyGameInstance.MyGameInstance_C|SetEnemy%20Targeted _mygameinstance 0)
        (bind _output_get (Variables|Default|SetIsTargeting false))
        (Development|PrintString (Utilities|String|Append "Targeting" (Utilities|String|ToString(Boolean) _output_get))))
      (:Is%20Not%20Valid
        (bind _output_get_2 (Variables|/Game/_Alex/Blueprints/Utility/MyGameInstance.MyGameInstance_C|SetEnemy%20Targeted _mygameinstance (Utilities|Array|Get(acopy) _enemies_in_range)))
        (for _array_element _enemies_in_range
          (Math|Float|CompareFloat (Transformation|GetDistanceTo _array_element _self) (Transformation|GetDistanceTo _output_get_2 _self)
            (:==
              _)
            (:<
              _))
          (Variables|/Game/_Alex/Blueprints/Utility/MyGameInstance.MyGameInstance_C|SetEnemy%20Targeted (Variables|Default|GetMyGameInstance) _array_element)
          (Variables|Default|SetIsTargeting true))))))

(event Input|ActionEvents|InputActionSlow
  (params (Key :type Key%20Structure))
  (:Pressed
    (Animation|Montage|PlayMontage (Variables|Character|GetMesh) "/Game/_Alex/Animations/Characters/Fusion/Attack/AM_Charge.AM_Charge"
      (:OnInterrupted
        (Development|PrintString "STOP"))))
  (:Released
    (Animation|StopAnimMontage 0)))

(event Input|ActionEvents|InputActionRotateAttack
  (params (Key :type Key%20Structure))
  ;[1 1 1] Attack Rotation
  (:Pressed
    (if (< (Variables|Default|GetAttackIndex) (Utilities|Array|LastIndex (Variables|Default|GetAttacks)))
      (Math|Integer|IncrementInt (Variables|Default|GetAttackIndex))
      (else
        (Variables|Default|SetAttackIndex 0)))))

(event Input|KeyboardEvents|P
  (params (Key :type Key%20Structure))
  ;[1 0.07684 0] DEBUG show enemy in range list
  (:Pressed
    (Development|PrintString (Utilities|String|ToString(Integer) (Variables|Default|GetAttackIndex)))))

(fn ConstructionScript)