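; BP_BlockPhysic is a breakable blocking wall that a BP_Ball in physics mode can destroy.
; Its trigger box is sized slightly larger than BlockingWall, in both the construction script and BeginPlay, to detect the ball around the wall.
; On overlap, the actor destroys itself if the ball has physics on and its speed is at least BreakableVelocity.
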(event OnComponentBeginOverlap(Trigger)
  (params (OverlappedComponent :type Primitive%20Component%20Object%20Reference) (OtherActor :type Actor%20Object%20Reference) (OtherComp :type Primitive%20Component%20Object%20Reference) (OtherBodyIndex :type Integer) (bFromSweep :type Boolean) (SweepResult :type Hit%20Result%20Structure%20%28by%20ref%29))
  ;[1 1 1] Destroy actor when the Ball in physic mode overlaps
  (bind _asbp_ball (Utilities|Casting|CastToBP_Ball OtherActor))
  (if (Variables|/Game/_Alex/Blueprints/Character/BP_Ball.BP_Ball_C|GetPhysicOn _asbp_ball)
    (Math|Float|CompareFloat (Math|Vector|VectorLength (Transformation|GetVelocity _asbp_ball)) (Variables|Default|GetBreakable%20Velocity)
      (:>
        _)
      (:==
        _))
    (Actor|DestroyActor)))

(event EventBeginPlay
  (Components|Box|SetBoxExtent (Variables|Default|GetTrigger) (* (Variables|/Script/Engine.BoxComponent|GetBoxExtent (Variables|Default|GetBlocking%20Wall)) 1.2) true))

(event Collision|EventActorBeginOverlap
  (params (OtherActor :type Actor%20Object%20Reference)))

(event EventTick
  (params (DeltaSeconds :type Float%20%28single-precision%29)))

(fn ConstructionScript
  (Components|Box|SetBoxExtent (Variables|Default|GetTrigger) (* (Variables|/Script/Engine.BoxComponent|GetBoxExtent (Variables|Default|GetBlocking%20Wall)) 1.2) true))